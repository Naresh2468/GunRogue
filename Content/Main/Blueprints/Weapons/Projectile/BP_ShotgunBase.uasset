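; Base Blueprint for grabbable shotguns, extending a parent weapon with optional internal shell storage and an animated loading latch.
; With internal storage, matching ammo overlapping MagazineHitBox increments the count, is released from the player's grab and reset for pooling.
; Stored shells appear as mesh instances on numbered ammo_bone sockets.
; LoadRound chambers from storage or defers to the parent, and one firing mode overrides slide-stop behavior.
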(event `self.ReceiveBeginPlay`
  (`parent.ReceiveBeginPlay`)
  (`|ExecutionSequence`
    (:`then_0`
      (if (`self.HasInternalAmmoStorage`)
        (`ActorComponent.K2_DestroyComponent` (`self.SlideMagCollisionConstraint`))
        (else
          (`ActorComponent.K2_DestroyComponent` (`self.StoredAmmo`)))))
    (:`then_1`
      (if (not (`self.HasLatch`))
        (`ActorComponent.K2_DestroyComponent` (`self.LatchMesh`))))))

(event `/Game/Main/Blueprints/Data/Interfaces/Weapon/BPI_WeaponInterface.StopMovingSlide`
  ; Stop moving the slide. If firing mode is single we want the slide to stay where it is.
  (if (`|EnumEquality` (`self.SelectedFiringMode`) "NewEnumerator0")
    (set `self.IsSlideBeingHeld` false)
    (else
      (`parent.StopMovingSlide`))))

(event `self.MagazineHitBox.OnComponentBeginOverlap`
  (params (OverlappedComponent :type "PrimitiveComponent Object Reference") (OtherActor :type "Actor Object Reference") (OtherComp :type "PrimitiveComponent Object Reference") (OtherBodyIndex :type Integer) (bFromSweep :type Boolean) (SweepResult :type "HitResult Structure (by ref)"))
  ; Load overlapped magazine or ammo based on, if shotgun has internal storage
  (if (`self.HasInternalAmmoStorage`)
    (bind _asbp_ammo_base (cast `/Game/Main/Blueprints/Weapons/Magazines/Ammo/BP_AmmoBase` OtherActor))
    (`self.LoadAmmo` _asbp_ammo_base)
    (`self.MoveLatch`)
    (set `self.BulletFireSingleReload` true)))

(fn `AddSingleRound`
  (returns (Success :type Boolean))
  (if (< (`self.CurrentAmmoCount`) (`self.MaxAmmoCount`))
    (bind _result (`/Engine/EditorBlueprintResources/StandardMacros.IncrementInt` (`self.CurrentAmmoCount`))
      (:`  `
        (`KismetSystemLibrary.PrintString` (`KismetStringLibrary.Conv_IntToString` _result) true true (struct :`R` 0.234375 :`G` 0.007201 :`B` 0.00487 :`A` 1.0))
        (`self.UpdateAllAmmoInstances`)
        (return true)))
    (else
      (return false))))

(fn `LoadAmmo`
  (params (NewAmmo :type "/Game/Main/Blueprints/Weapons/Magazines/Ammo/BP_AmmoBase Object Reference"))
  (bind _newammo (`local.NewAmmo`))
  (`KismetSystemLibrary.IsObjectOfSoftClass` NewAmmo (`|ConvertAsset` (`self.MatchingAmmoClass`))
    (:`True`
      (bind _success (`self.AddSingleRound`))
      (if _success
        (message `/Game/Main/Blueprints/Data/System/AudioManager/SoundData/Interface/BPI_Audio.IE_PlaySFXSound` (`GameplayStatics.GetGameMode`) "NewEnumerator0" (`self.Weapon_InsertAmmo`) false (`SceneComponent.K2_GetComponentLocation` (`self.MagazineHitBox`)))
        (bind _player (message `/Game/Marketplace/ALS/Blueprints/Interfaces/BPI_Player.F_PlayerRef` (`GameplayStatics.GetPlayerCharacter` 0)))
        ; Ammo base of Shot Gun Ammo Pooling calling from here
        (`/Game/Main/Blueprints/Weapons/Magazines/Ammo/BP_AmmoBase.AmmoInUse` _newammo false)
        (`/Game/Main/Blueprints/Character/Player/BP_VRCharacter.ReleaseGrabbedActor` _player _newammo)
        (message `/Game/Main/Blueprints/Data/System/ObjectPooling/BP/Interface/BPI_Pooling.IE_ResetManual` _newammo)))))

(fn `LoadRound`
  (returns (CanReleaseSlide :type Boolean))
  (`/Engine/EditorBlueprintResources/StandardMacros.IsValid` (`self.LoadedAmmo`)
    (:`Is Valid`
      (return false))
    (:`Is Not Valid`
      (if (`self.HasInternalAmmoStorage`)
        (bind _success (`self.RemoveSingleRound`))
        (if _success
          (`self.SpawnLoadedRound` (`self.MatchingAmmoClass`))
          (return (`|EnumInequality` (`self.SelectedFiringMode`) "NewEnumerator0")))
        (else
          (bind _canreleaseslide (`parent.LoadRound`))
          (return _canreleaseslide))))))

(fn `MoveLatch`
  (`SceneComponent.K2_SetRelativeRotation` (`self.LatchMesh`) (`self.LatchRotationOffset`) false false)
  (`KismetSystemLibrary.K2_SetTimer` null "ResetLatch" (`self.LatchResetDelay`)))

(fn `RefillAmmo`
  (set `self.CurrentAmmoCount` (`self.MaxAmmoCount`))
  (`self.UpdateAllAmmoInstances`))

(fn `RemoveSingleRound`
  (returns (Success :type Boolean))
  (bind _currentammocount (`self.CurrentAmmoCount`))
  (bind _returnvalue (`InstancedStaticMeshComponent.GetInstanceCount` (`self.StoredAmmo`)))
  (if (> _currentammocount 0)
    ; Only remove an instance if the current ammo count is less than the physical ammo instances
    (bind _result (`/Engine/EditorBlueprintResources/StandardMacros.DecrementInt` _currentammocount)
      (:`  `
        (if (< _result _returnvalue)
          (`InstancedStaticMeshComponent.RemoveInstance` (`self.StoredAmmo`) (- _returnvalue 1)))
        (return true)))
    (else
      (return false))))

(fn `ResetLatch`
  (`SceneComponent.K2_SetRelativeRotation` :`self` (`self.LatchMesh`)))

(fn `UpdateAllAmmoInstances`
  (`InstancedStaticMeshComponent.ClearInstances` (`self.StoredAmmo`))
  ; Adds an ammo instance for every instance of a found ammo bone
  (for _index (range (`self.CurrentAmmoCount`))
    (bind _returnvalue (`KismetStringLibrary.Conv_StringToName` (`KismetStringLibrary.Concat_StrStr` "ammo_bone_" (`KismetStringLibrary.Conv_IntToString` _index))))
    (if (`SceneComponent.DoesSocketExist` (`self.WeaponMesh`) _returnvalue)
      (`InstancedStaticMeshComponent.AddInstance` (`self.StoredAmmo`) (`SceneComponent.GetSocketTransform` (`self.WeaponMesh`) _returnvalue "RTS_Component") false))))

(fn `UserConstructionScript`
  (`parent.UserConstructionScript`))