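; BP_AmmoBoxBase is a base ammo box that hands out one round at a time for a character to hold.
; TakeAmmo removes a round from the count, spawns an ammo actor, snaps it to the given character mesh bone and sets its meshes to overlap collision.
; It allows only one spawned round at a time.
; ReturnAmmo adds the round back and destroys the actor through ClearSpawnedAmmo.
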(fn `ClearSpawnedAmmo`
  (bind _spawnedammo (`self.SpawnedAmmo`))
  (`|ExecutionSequence`
    (:`then_0`
      (`/Engine/EditorBlueprintResources/StandardMacros.IsValid` _spawnedammo
        (:`Is Valid`
          (`self.K2_DestroyActor` _spawnedammo))))
    (:`then_1`
      (set `self.SpawnedAmmo` null))))

(fn `ReturnAmmo`
  (`/Engine/EditorBlueprintResources/StandardMacros.IsValid` (`self.SpawnedAmmo`)
    (:`Is Valid`
      (`self.AddSingleRound`)
      (`self.ClearSpawnedAmmo`))))

(fn `TakeAmmo`
  (params (CharacterMesh :type "SkeletalMeshComponent Object Reference") (BoneToAttachTo :type Name))
  (returns (AmmoActor :type "Actor Object Reference"))
  (`/Engine/EditorBlueprintResources/StandardMacros.IsValid` (`self.SpawnedAmmo`)
    (:`Is Valid`
      (return null))
    (:`Is Not Valid`
      (bind _wasammoremoved (`self.RemoveSingleRound`))
      (if _wasammoremoved
        (bind _returnvalue (`|SpawnActorFromClass` (`self.AmmoClass`) (`KismetMathLibrary.MakeTransform` (0.0 0.0 0.0)) "AlwaysSpawn" "MultiplyWithRoot" null null))
        (`/Engine/EditorBlueprintResources/StandardMacros.IsValid` _returnvalue
          (:`Is Valid`
            (bind _output_get (set `self.SpawnedAmmo` _returnvalue))
            (`self.SetOwner` _output_get self)
            (`self.K2_AttachToComponent` (`self.SpawnedAmmo`) (`local.CharacterMesh`) (`local.BoneToAttachTo`) "SnapToTarget" "SnapToTarget" "KeepRelative" true)
            (`PrimitiveComponent.SetCollisionResponseToAllChannels` (`/Game/Main/Blueprints/Weapons/Magazines/Ammo/BP_AmmoBase.AmmoMesh` (`self.SpawnedAmmo`)) "ECR_Overlap")
            (`PrimitiveComponent.SetCollisionResponseToAllChannels` (`/Game/Main/Blueprints/Weapons/Magazines/Ammo/BP_AmmoBase.ShotAmmoMesh` (`self.SpawnedAmmo`)) "ECR_Overlap")
            (return (`self.SpawnedAmmo`)))
          (:`Is Not Valid`
            (return null)))
        (else
          (return null))))))

(fn `UserConstructionScript`)