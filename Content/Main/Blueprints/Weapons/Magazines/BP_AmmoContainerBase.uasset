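; Base ammo container for weapon magazines that tracks the round count and shows the loaded rounds, filling to capacity on BeginPlay.
; Refilling or adding a round rebuilds StoredAmmo mesh instances on numbered ammo_bone_ sockets, so only rounds with a matching socket are drawn.
; Removing a round lowers the count and drops the last instance only once the count falls below the visible instances.
; Debug events wrap refill, single removal and full emptying.
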(event `self.ReceiveBeginPlay`
  (`self.RefillMag`))

(event `DebugRemoveBullet`
  ; DEBUG
  (`self.RemoveSingleRound`))

(event `DebugRefillMagazine`
  ; DEBUG
  (`self.RefillMag`))

(event `DebugRemoveAllBullet`
  (`self.RemoveAllRound`))

(fn `AddSingleRound`
  (bind _currentammocount (`self.CurrentAmmoCount`))
  (bind _maxammocount (`self.MaxAmmoCount`))
  (if (< _currentammocount _maxammocount)
    (`/Engine/EditorBlueprintResources/StandardMacros.IncrementInt` _currentammocount
      (:`  `
        _))
    (else
      (set `self.CurrentAmmoCount` _maxammocount)))
  (`self.UpdateAllAmmoInstances`))

(fn `RefillMag`
  (set `self.CurrentAmmoCount` (`self.MaxAmmoCount`))
  (`self.UpdateAllAmmoInstances`))

(fn `RemoveAllRound`
  (returns (WasAmmoRemoved :type Boolean))
  (if (> (`self.CurrentAmmoCount`) 0)
    (bind _output_get (set `self.Total Ammo` (- (`InstancedStaticMeshComponent.GetInstanceCount` (`self.StoredAmmo`)) 1)))
    (for _ (range (+ _output_get 1))
      (`InstancedStaticMeshComponent.RemoveInstance` (`self.StoredAmmo`) (- (`InstancedStaticMeshComponent.GetInstanceCount` (`self.StoredAmmo`)) 1)))
    (set `self.CurrentAmmoCount` 0)
    (return true)))

(fn `RemoveSingleRound`
  (returns (WasAmmoRemoved :type Boolean))
  (bind _returnvalue (`InstancedStaticMeshComponent.GetInstanceCount` (`self.StoredAmmo`)))
  (if (> (`self.CurrentAmmoCount`) 0)
    (bind _result (`/Engine/EditorBlueprintResources/StandardMacros.DecrementInt` (`self.CurrentAmmoCount`))
      (:`  `
        (if (< _result _returnvalue)
          (`InstancedStaticMeshComponent.RemoveInstance` (`self.StoredAmmo`) (- _returnvalue 1)))
        (return true)))
    (else
      (return false))))

(fn `UpdateAllAmmoInstances`
  (`InstancedStaticMeshComponent.ClearInstances` (`self.StoredAmmo`))
  (for _index (range (`self.CurrentAmmoCount`))
    (bind _returnvalue (`KismetStringLibrary.Conv_StringToName` (`KismetStringLibrary.Concat_StrStr` "ammo_bone_" (`KismetStringLibrary.Conv_IntToString` _index))))
    (if (`SceneComponent.DoesSocketExist` (`self.Mesh`) _returnvalue)
      (`InstancedStaticMeshComponent.AddInstance` (`self.StoredAmmo`) (`SceneComponent.GetSocketTransform` (`self.Mesh`) _returnvalue "RTS_Component") false))))

(fn `UserConstructionScript`)