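; Base bullet projectile that applies damage on mesh hit and destroys itself on impact or when its lifetime timer expires.
; Hits send damage and hit reaction messages to the struck actor, always crediting player 0 as causer.
; DestroyProjectile plays the impact sound and attaches a decal, or only the sound for explosive rounds that time out.
; Impact particle spawns are present but disconnected, so they never run.
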(event `self.ReceiveBeginPlay`
  (bind _returnvalue (`KismetSystemLibrary.K2_SetTimerDelegate` (delegate `OnProjectileLifetimeExpired`) (`self.Lifetime`)))
  (set `self.LifetimeTH` _returnvalue))

(event `OnProjectileLifetimeExpired`
  (`self.DestroyProjectile` (struct)))

(event `self.BulletMesh.OnComponentHit`
  (params (HitComponent :type "PrimitiveComponent Object Reference") (OtherActor :type "Actor Object Reference") (OtherComp :type "PrimitiveComponent Object Reference") (NormalImpulse :type "Vector Structure") (Hit :type "HitResult Structure (by ref)"))
  (bind (_bblockinghit _binitialoverlap _time _distance _location _impactpoint _normal _impactnormal _physmat _hitactor _hitcomponent _hitbonename) (`GameplayStatics.BreakHitResult` Hit))
  (bind _damage_amount (`self.Damage Amount`))
  (`self.DestroyProjectile` Hit)
  (message `/Game/Main/Blueprints/Data/Interfaces/Gameplay/HealthDamage/BPI_Damageable.F_TakeDamage` _hitactor (make `/Game/Main/Blueprints/Data/Struct/Character/Damage/S_DamageInfo` _damage_amount "NewEnumerator2" "NewEnumerator1") (`GameplayStatics.GetPlayerCharacter` 0) Hit)
  (message `/Game/Marketplace/ALS/Blueprints/Interfaces/Enemy_BPI.HitReaction` _hitactor _impactpoint _hitbonename (`self.Hit Strength`) _damage_amount))

(fn `DestroyProjectile`
  (params (Hit :type "HitResult Structure"))
  (locals (HitComponent :type "PrimitiveComponent Object Reference") (HitLocation :type "Vector Structure") (ImpactRotation :type "Rotator Structure" :default (struct)) (HitBone :type Name))
  (bind (_bblockinghit _binitialoverlap _time _distance _location _impactpoint _normal _impactnormal _physmat _hitactor _hitcomponent _hitbonename) (`GameplayStatics.BreakHitResult` Hit))
  (`|ExecutionSequence`
    (:`then_0`
      (`KismetSystemLibrary.K2_ClearAndInvalidateTimerHandle` (`self.LifetimeTH`))
      (bind _output_get (set `local.HitComponent` _hitcomponent))
      (`/Engine/EditorBlueprintResources/StandardMacros.IsValid` _output_get
        (:`Is Valid`
          (set `local.HitLocation` _location)
          (set `local.ImpactRotation` (`KismetMathLibrary.Conv_VectorToRotator` _impactnormal))
          (set `local.HitBone` _hitbonename)
          ; Impact particles, sound and decal
          (`GameplayStatics.PlaySoundAtLocation` (`self.ImpactSound`) (`local.HitLocation`) (struct) 1.0 1.0 0.0 null null null null)
          (`GameplayStatics.SpawnDecalAttached` (`self.ImpactDecal`) (3.0 3.0 3.0) (`local.HitComponent`) (`local.HitBone`) (`local.HitLocation`) (`local.ImpactRotation`) "KeepWorldPosition" 10.0))
        (:`Is Not Valid`
          ; Used when the lifetime timer expires and the projectile is explosive, like a missile
          (if (`self.IsExplosive`)
            (`GameplayStatics.PlaySoundAtLocation` (`self.ImpactSound`) (`self.K2_GetActorLocation`) (struct) 1.0 1.0 0.0 null null null null)))))
    (:`then_1`
      (`self.K2_DestroyActor`))))

(fn `UserConstructionScript`)