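; Base actor for a single ammo round in a motion-controller weapon system, swapping from the live mesh to a shot mesh once fired.
; Interface events store pooling data and the holding controller, though the return-to-pool call is unwired and despawning destroys the actor after a delay.
; In-use changes request haptics from the GameMode; release first clears the controller, hides the round and disables its collision and overlaps.
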(event `self.ReceiveBeginPlay`
  (`SceneComponent.SetVisibility` (`self.ShotAmmoMesh`) false false))

(event `DespawnAmmo`
  (`KismetSystemLibrary.Delay` (`self.DelayDestroy`))
  (`self.K2_DestroyActor`))

(event `/Game/Main/Blueprints/Data/System/ObjectPooling/BP/Interface/BPI_Pooling.IE_SetInfo`
  (params (TimeToAlive :type "Float (double-precision)") (DefaultLocation :type "Vector Structure"))
  ; Pooling Actor data
  (set `self.Time to Alive` TimeToAlive)
  (set `self.Default Location` DefaultLocation))

(event `/Game/Main/Blueprints/Data/System/ObjectPooling/BP/Interface/BPI_Pooling.IE_SetInuse`
  (params (isUse :type Boolean))
  ; Pooling Actor data
  (set `self.Is Use` isUse))

(event `AmmoInUse`
  (params (AmmoInused :type Boolean))
  (bind _output_get (set `self.AmmoInused` AmmoInused))
  (if (not _output_get)
    (set `self.Motion Controller` null)
    (`self.SetActorHiddenInGame` true)
    (`self.F_MeshCollision` false))
  (`self.AmmoHapticEffect`))

(event `/Game/Main/Blueprints/Data/Interfaces/Weapon/Ammo/BPI_AmmoPick.IE_CurrentAmmo`
  (params (CurrentGun :type Name) (AmmoSpawnTransform :type "Transform Structure") (MotionController :type "MotionControllerComponent Object Reference"))
  (set `self.Motion Controller` MotionController))

(event `AmmoHapticEffect`
  (message `/Game/Main/Blueprints/Data/Interfaces/Mode/BPI_GMMain.IE_HapticEffect` (`GameplayStatics.GetGameMode`) (`self.Motion Controller`) "NewEnumerator0"))

(fn `F_GetClass`
  (returns (ClassRef :type "Actor Class Reference"))
  (return (`GameplayStatics.GetObjectClass` self)))

(fn `F_GetData`
  (returns (`Is usedActor` :type Boolean) (DefaultLocation :type "Vector Structure"))
  (return (`self.Is Use`) (`self.Default Location`)))

(fn `F_MeshCollision`
  (params (Toggle :type Boolean))
  (bind _shotammomesh (`self.ShotAmmoMesh`))
  (bind _ammomesh (`self.AmmoMesh`))
  (`PrimitiveComponent.SetCollisionResponseToChannel` _shotammomesh "ECC_GameTraceChannel1" (select `bool` Toggle :`false` "ECR_Ignore" :`true` "ECR_Block" :!type "ECollisionResponse Enum"))
  (`PrimitiveComponent.SetCollisionResponseToChannel` _ammomesh "ECC_Visibility" (select `bool` Toggle :`false` "ECR_Ignore" :`true` "ECR_Block" :!type "ECollisionResponse Enum"))
  (`PrimitiveComponent.SetCollisionResponseToChannel` _shotammomesh "ECC_Visibility" (select `bool` Toggle :`false` "ECR_Ignore" :`true` "ECR_Block" :!type "ECollisionResponse Enum"))
  (`PrimitiveComponent.SetCollisionObjectType` _ammomesh (select `bool` Toggle :`false` "ECC_WorldStatic" :`true` "ECC_GameTraceChannel1" :!type "ECollisionChannel Enum"))
  (`PrimitiveComponent.SetCollisionObjectType` _shotammomesh (select `bool` Toggle :`false` "ECC_WorldStatic" :`true` "ECC_GameTraceChannel1" :!type "ECollisionChannel Enum"))
  (set `PrimitiveComponent.bGenerateOverlapEvents` Toggle _ammomesh)
  (set `PrimitiveComponent.bGenerateOverlapEvents` Toggle _shotammomesh))

(fn `IE_GetSpawnID`
  (returns (SpawnID :type Name))
  (return "None"))

(fn `SetAmmoShot`
  (set `self.WasShot` true)
  (`SceneComponent.SetVisibility` (`self.AmmoMesh`) false false)
  (`SceneComponent.SetVisibility` (`self.ShotAmmoMesh`) true false))

(fn `UserConstructionScript`)