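; BP_RifleMagPool is a pooled rifle magazine actor that returns itself to the game mode's pool when left unused.
; Setting it in use switches mesh physics simulation on, and releasing it switches simulation off.
; A manual reset waits out an alive timer, rechecks that it is still unused, then messages the game mode, restores mesh collision and refills the ammo.
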(event `/Game/Main/Blueprints/Data/System/ObjectPooling/BP/Interface/BPI_Pooling.IE_SetInuse`
  (params (isUse :type Boolean))
  (bind _mesh (`self.Mesh`))
  (`parent.IE_SetInuse` isUse)
  (if isUse
    (`PrimitiveComponent.SetSimulatePhysics` _mesh true)
    (else
      (`PrimitiveComponent.SetSimulatePhysics` _mesh false))))

(event `/Game/Main/Blueprints/Data/System/ObjectPooling/BP/Interface/BPI_Pooling.IE_ResetManual`
  (if (not (`self.MagazineInuse`))
    (`KismetSystemLibrary.Delay` (`self.Time to Alive`))
    (if (not (`self.MagazineInuse`))
      (message `/Game/Main/Blueprints/Data/Interfaces/Mode/BPI_GMMain.IE_ReturnToPool` (`GameplayStatics.GetGameMode`) self)
      (`self.F_MeshCollision` true)
      (`self.RefillMag`))))

(fn `UserConstructionScript`
  (`parent.UserConstructionScript`))