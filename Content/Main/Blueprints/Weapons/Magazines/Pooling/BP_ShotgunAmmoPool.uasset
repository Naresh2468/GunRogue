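; Pooled shotgun ammo actor, built on a parent class that supplies the base in-use handling.
; When taken into use it unhides and enables AmmoMesh physics a tick later; when released it hides and stops simulating.
; A manual reset waits out its alive time, then, if the ammo is not marked used, sends the GameMode a return-to-pool message and calls the mesh collision function.
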(event `/Game/Main/Blueprints/Data/System/ObjectPooling/BP/Interface/BPI_Pooling.IE_SetInuse`
  (params (isUse :type Boolean))
  (bind _ammomesh (`self.AmmoMesh`))
  ; IMP Step
  (`parent.IE_SetInuse` isUse)
  (`self.SetActorHiddenInGame` (not isUse))
  (if isUse
    (`KismetSystemLibrary.DelayUntilNextTick`)
    (`PrimitiveComponent.SetSimulatePhysics` _ammomesh true)
    (else
      (`PrimitiveComponent.SetSimulatePhysics` _ammomesh false))))

(event `/Game/Main/Blueprints/Data/System/ObjectPooling/BP/Interface/BPI_Pooling.IE_ResetManual`
  (`KismetSystemLibrary.Delay` (`self.Time to Alive`))
  (if (not (`self.AmmoInused`))
    (message `/Game/Main/Blueprints/Data/Interfaces/Mode/BPI_GMMain.IE_ReturnToPool` (`GameplayStatics.GetGameMode`) self)
    (`self.F_MeshCollision` true)))

(fn `UserConstructionScript`
  (`parent.UserConstructionScript`))