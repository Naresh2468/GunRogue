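; Base magazine Blueprint for motion-controller weapons, built to work as a pooled actor with in-use state, visibility and a default location.
; When a magazine goes in use, it disables mesh collision and requests haptics through the GameMode; otherwise it clears its MotionController.
; Overrides of the parent's ammo functions move the carry mesh to the carry_bone socket matching the stored round count.
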(event `/Game/Main/Blueprints/Data/System/ObjectPooling/BP/Interface/BPI_Pooling.IE_SetInfo`
  (params (TimeToAlive :type "Float (double-precision)") (DefaultLocation :type "Vector Structure"))
  ; Pooling Actor data
  (set `self.Time to Alive` TimeToAlive)
  (set `self.Default Location` DefaultLocation))

(event `/Game/Main/Blueprints/Data/System/ObjectPooling/BP/Interface/BPI_Pooling.IE_SetInuse`
  (params (isUse :type Boolean))
  ; Pooling Actor data
  (bind _output_get (set `self.Is Use` isUse))
  (`self.SetActorHiddenInGame` (not _output_get)))

(event `MagazineActiveToggle`
  (params (MagazineInuse :type Boolean))
  (bind _output_get (set `self.MagazineInuse` MagazineInuse))
  ; Make sure reset Actor to default cause it may create issue to other attempt interaction
  (if _output_get
    (`self.F_MeshCollision` false)
    (`self.AmmoHapticEffect`)
    (`KismetSystemLibrary.PrintString` "Collision Off" true true (struct :`R` 1.0 :`B` 0.175058 :`A` 1.0) :!enabledstate Disabled)
    (else
      (set `self.MotionController` null))))

(event `/Game/Main/Blueprints/Data/Interfaces/Weapon/Ammo/BPI_AmmoPick.IE_CurrentAmmo`
  (params (CurrentGun :type Name) (AmmoSpawnTransform :type "Transform Structure") (MotionController :type "MotionControllerComponent Object Reference"))
  (set `self.MotionController` MotionController))

(event `AmmoHapticEffect`
  (message `/Game/Main/Blueprints/Data/Interfaces/Mode/BPI_GMMain.IE_HapticEffect` (`GameplayStatics.GetGameMode`) (`self.MotionController`) "NewEnumerator0"))

(fn `F_GetClass`
  (returns (ClassRef :type "Actor Class Reference"))
  (return (`GameplayStatics.GetObjectClass` self)))

(fn `F_GetData`
  (returns (`Is usedActor` :type Boolean) (DefaultLocation :type "Vector Structure"))
  (return (`self.Is Use`) (`self.Default Location`)))

(fn `F_MeshCollision`
  (params (Toggle :type Boolean))
  (bind _mesh (`self.Mesh`))
  (`PrimitiveComponent.SetCollisionResponseToChannel` _mesh "ECC_GameTraceChannel1" (select `bool` Toggle :`false` "ECR_Ignore" :`true` "ECR_Block" :!type "ECollisionResponse Enum"))
  (`PrimitiveComponent.SetCollisionResponseToChannel` _mesh "ECC_Visibility" (select `bool` Toggle :`false` "ECR_Ignore" :`true` "ECR_Block" :!type "ECollisionResponse Enum"))
  (`PrimitiveComponent.SetCollisionObjectType` _mesh (select `bool` Toggle :`false` "ECC_WorldStatic" :`true` "ECC_GameTraceChannel1" :!type "ECollisionChannel Enum")))

(fn `IE_GetSpawnID`
  (returns (SpawnID :type Name))
  (return "None"))

(fn `RefillMag`
  (`parent.RefillMag`)
  (`self.UpdateCarryPosition`))

(fn `RemoveSingleRound`
  (returns (WasAmmoRemoved :type Boolean))
  (bind _wasammoremoved (`parent.RemoveSingleRound`))
  (`self.UpdateCarryPosition`)
  (return _wasammoremoved))

(fn `UpdateAllAmmoInstances`
  (`parent.UpdateAllAmmoInstances`)
  (`self.UpdateCarryPosition`))

(fn `UpdateCarryPosition`
  (bind _returnvalue (`KismetStringLibrary.Conv_StringToName` (`KismetStringLibrary.Concat_StrStr` "carry_bone_" (`KismetStringLibrary.Conv_IntToString` (- (`InstancedStaticMeshComponent.GetInstanceCount` (`self.StoredAmmo`)) 1)))))
  (if (`SceneComponent.DoesSocketExist` (`self.Mesh`) _returnvalue)
    (`SceneComponent.K2_SetRelativeTransform` (`self.CarryMesh`) (`SceneComponent.GetSocketTransform` (`self.Mesh`) _returnvalue "RTS_Component") false true)))

(fn `UserConstructionScript`)