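; BP_WeaponLoadout is an actor that spawns the player's unlocked weapons when play begins.
; It fetches weapon upgrade data from the Game Instance through a fetch-data call and spawns the class of each entry marked unlocked.
; The M_SpawnTransform macro supplies placement, with nodes for offsetting along the actor's forward vector by spawn count and Distance, using the SpawnPoint component's rotation.
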(event `self.ReceiveBeginPlay`
  (`self.F_WeaponLoadout`))

(fn `F_WeaponLoadout`
  (bind (_location _rotation) (`self.M_SpawnTransform`))
  (bind (_gameplaydata _weaponupgrade) (message `/Game/Main/Blueprints/Data/Interfaces/SaveGame/BPI_SaveGame.IE_FetchData` (`GameplayStatics.GetGameInstance`)))
  (for _array_element _weaponupgrade
    (bind ((`WeaponUnlockReason_51_197419EB46085B05353351A5A5CFCD63` _weaponunlockreason) (`WeaponUnlocked_23_C701FB2B47EB29FD05F3A29810DFDD4A` _weaponunlocked) (`WeaponClass_42_2D05F92842E0DEBD8EEC93892B5C0E99` _weaponclass)) (break `/Game/Main/Blueprints/Data/Struct/Upgrade/S_UpgradeInformation` _array_element))
    (if _weaponunlocked
      (`|SpawnActorFromClass` _weaponclass (`KismetMathLibrary.MakeTransform` _location _rotation) "Undefined" "MultiplyWithRoot" null null)
      (set `self.WeaponUpdate` (+ (`self.WeaponUpdate`) 1))
      (else
        (`KismetSystemLibrary.PrintString` "Failed TO fetch" true true (struct :`R` 1.0 :`G` 0.115418 :`A` 1.0) :!enabledstate Disabled))))
  (set `self.WeaponUpdate` 0))

(fn `UserConstructionScript`)