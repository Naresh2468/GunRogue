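; Tutorial weapon loadout actor that spawns a weapon actor for each weapon upgrade entry fetched from the Game Instance.
; It spawns the set on BeginPlay, using a transform macro that appears to space weapons along the actor's forward vector by a running counter.
; It also binds to the Game State event manager's reload-loadout dispatcher, spawning the set again after a short delay without removing earlier spawns.
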(event `self.ReceiveBeginPlay`
  (`self.F_WeaponLoadout`)
  (bind _gamestate (message `/Game/Main/Blueprints/Data/Interfaces/EventManager/BPI_GameStateEvents.F_EventManagerRef` (`GameplayStatics.GetGameState`)))
  (add `/Game/Main/Blueprints/Data/Gamestate/GS_Main.ED_ReloadLoadOut` _gamestate (delegate `ReloadLoadOutWeapons`)))

(event `ReloadLoadOutWeapons`
  (`KismetSystemLibrary.Delay` 0.1)
  (`self.F_WeaponLoadout`))

(fn `F_WeaponLoadout`
  (bind (_location _rotation) (`self.M_SpawnTransform`))
  (bind (_gameplaydata _weaponupgrade) (message `/Game/Main/Blueprints/Data/Interfaces/SaveGame/BPI_SaveGame.IE_FetchData` (`GameplayStatics.GetGameInstance`)))
  (for _array_element _weaponupgrade
    (`|SpawnActorFromClass` (`.WeaponClass_42_2D05F92842E0DEBD8EEC93892B5C0E99` (break `/Game/Main/Blueprints/Data/Struct/Upgrade/S_UpgradeInformation` _array_element)) (`KismetMathLibrary.MakeTransform` _location _rotation) "Undefined" "MultiplyWithRoot" null null)
    (set `self.WeaponUpdate` (+ (`self.WeaponUpdate`) 1)))
  (set `self.WeaponUpdate` 0))

(fn `UserConstructionScript`)