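; Base weapon Blueprint with experimental physics-based penetration for sharp melee weapons; blunt types destroy those components at BeginPlay.
; Fast enough hitbox overlaps with "penetrable"-tagged actors constrain the mesh to the hit component and bone.
; The breakable constraint reattaches while that target remains set; end overlap clears it and releases.
; Also provides display-marker toggles and default gun getters; damage and impact effects are unimplemented or disconnected.
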(event `self.ReceiveBeginPlay`
  (bind _penetrationconstraint (`self.PenetrationConstraint`))
  (switch `/Game/Main/Blueprints/Weapons/E_WeaponMeleeType` (`self.WeaponMeleeType`)
    (:`NewEnumerator0`
      (`ActorComponent.K2_DestroyComponent` (`self.PenetrationHitBox`))
      (`ActorComponent.K2_DestroyComponent` (`self.PenetrationConstraint`)))
    (:`NewEnumerator1`
      (add `PhysicsConstraintComponent.OnConstraintBroken` _penetrationconstraint (delegate `OnConstraintBroken`))
      (`PhysicsConstraintComponent.SetLinearBreakable` _penetrationconstraint true (`self.LinearBreakForce`)))))

(event `OnConstraintBroken`
  (params (ConstraintIndex :type Integer))
  (bind _penetratedcomponent (`self.PenetratedComponent`))
  (`/Engine/EditorBlueprintResources/StandardMacros.IsValid` _penetratedcomponent
    (:`Is Valid`
      (`PhysicsConstraintComponent.SetConstrainedComponents` (`self.PenetrationConstraint`) (`self.WeaponMesh`) "None" _penetratedcomponent (`self.PenetratedBone`)))))

(event `self.WeaponMesh.OnComponentHit`
  (params (HitComponent :type "PrimitiveComponent Object Reference") (OtherActor :type "Actor Object Reference") (OtherComp :type "PrimitiveComponent Object Reference") (NormalImpulse :type "Vector Structure") (Hit :type "HitResult Structure (by ref)"))
  ; Mesh Hit Event
  (`/Engine/EditorBlueprintResources/StandardMacros.IsValid` (`self.GetOwner`)
    (:`Is Valid`
      (`/Engine/EditorBlueprintResources/StandardMacros.IsValid` (`self.PenetratedComponent`)))))

(event `self.PenetrationHitBox.OnComponentBeginOverlap`
  (params (OverlappedComponent :type "PrimitiveComponent Object Reference") (OtherActor :type "Actor Object Reference") (OtherComp :type "PrimitiveComponent Object Reference") (OtherBodyIndex :type Integer) (bFromSweep :type Boolean) (SweepResult :type "HitResult Structure (by ref)"))
  (bind _returnvalue (`self.GetOwner`))
  ; Blade and Tip Overlap Events (Experimental)
  (`/Engine/EditorBlueprintResources/StandardMacros.IsValid` _returnvalue
    (:`Is Valid`
      (if (and (`self.ActorHasTag` OtherActor "penetrable") (!= OtherActor _returnvalue))
        (set `self.OverlappedPenetrableActor` OtherActor)
        (bind _returnvalue_2 (`PrimitiveComponent.GetPhysicsLinearVelocity` (`self.WeaponMesh`) "None"))
        (if (> (* (`KismetMathLibrary.VSize` _returnvalue_2) (`GameplayStatics.GetWorldDeltaSeconds`)) (`self.MinPenetrationSpeed`))
          (`self.SetPenetrationConstraint` OtherComp (`.HitBoneName` (`GameplayStatics.BreakHitResult` SweepResult))))))))

(event `self.PenetrationHitBox.OnComponentEndOverlap`
  (params (OverlappedComponent :type "PrimitiveComponent Object Reference") (OtherActor :type "Actor Object Reference") (OtherComp :type "PrimitiveComponent Object Reference") (OtherBodyIndex :type Integer))
  ; Blade and Tip Overlap Events (Experimental)
  (if (== OtherActor (`self.OverlappedPenetrableActor`))
    (set `self.OverlappedPenetrableActor` null)
    (set `self.PenetratedComponent` null)
    (set `self.PenetratedBone` "None")
    (`PhysicsConstraintComponent.BreakConstraint` (`self.PenetrationConstraint`))))

(event `/Game/Main/Blueprints/Data/Interfaces/UMG/Marker/BPI_Marker.IE_ToggleDisplayMaker`
  (params (ToggleMarker :type Boolean))
  (bind _bpsc_displaymarker (`self.BPSC_DisplayMarker`))
  (if ToggleMarker
    (if (not (`self.IsStopDisplay`))
      (`/Game/Main/Blueprints/Data/Component/BPSC_DisplayMarker.DisplayMarker` _bpsc_displaymarker))
    (else
      (`/Game/Main/Blueprints/Data/Component/BPSC_DisplayMarker.StopMarker` _bpsc_displaymarker))))

(event `/Game/Main/Blueprints/Data/Interfaces/Weapon/BPI_WeaponInterface.IE_MarkerHandler`
  (params (Toggle :type Boolean))
  (set `self.IsStopDisplay` Toggle))

(fn `CheckInterval`
  (params (Value :type "Float (double-precision)") (Interval :type "Float (double-precision)"))
  (returns (IsInInterval :type Boolean))
  (return (>= (- (`GameplayStatics.GetTimeSeconds`) Value) Interval)))

(fn `DealDamage`
  (params (ActorToDamage :type "Actor Object Reference") (DamageType :type "/Game/Main/Blueprints/Weapons/E_DamageType Enum" :default "NewEnumerator0")))

(fn `F_CanFire`
  (returns (CanEffect :type Boolean))
  (return false))

(fn `F_CurrentGunData`
  (returns (GunName :type Name))
  (return (`self.CurrentGunName`)))

(fn `F_GetProjectileType`
  (returns (ProjectileType :type "/Game/Main/Blueprints/Weapons/E_ProjectileWeaponType Enum"))
  (return (`self.ProjectileWeaponType`)))

(fn `F_WeaponRef`
  (returns (CurrentWeapon :type "/Game/Main/Blueprints/Weapons/BP_WeaponBase Object Reference"))
  (return self))

(fn `GetSlideComponent`
  (returns (SlideComponent :type "PrimitiveComponent Object Reference"))
  (return null))

(fn `SetPenetrationConstraint`
  (params (ComponentToConstrain :type "PrimitiveComponent Object Reference") (BoneToConstrain :type Name))
  (set `self.PenetratedComponent` ComponentToConstrain)
  (set `self.PenetratedBone` BoneToConstrain)
  (`PhysicsConstraintComponent.SetConstrainedComponents` (`self.PenetrationConstraint`) (`self.WeaponMesh`) "None" ComponentToConstrain BoneToConstrain))

(fn `UserConstructionScript`)