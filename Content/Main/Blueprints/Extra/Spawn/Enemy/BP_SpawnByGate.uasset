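; Trigger gate that spawns enemies when the player overlaps its box, if the game mode's spawn-by-gate setting is on.
; On first overlap, it asks the GameMode to spawn an enemy at each spawn point, setting state and spawn ID, then disables collision on linked gates.
; ResetElement re-enables collision and both DoOnce latches, while BeginPlay registers with the event manager's actor reset.
; Editor events create and clear attached spawn point actors.
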(event `self.ReceiveBeginPlay`
  (bind _gamestate (message `/Game/Main/Blueprints/Data/Interfaces/EventManager/BPI_Events.F_EventManagerRef` (`GameplayStatics.GetGameState`)))
  (`/Engine/EditorBlueprintResources/StandardMacros.IsValid` _gamestate
    (:`Is Valid`
      (add `/Game/Main/Blueprints/Data/Gamestate/GS_Main.ED_GameActorReset` _gamestate (`|CreateDelegate` :!event `ResetElement`)))))

(event `ResetElement`
  (`self.ResetCollision`)
  (`self.ResetCollisionOther`))

(event `self.Box.OnComponentBeginOverlap`
  (params (OverlappedComponent :type "PrimitiveComponent Object Reference") (OtherActor :type "Actor Object Reference") (OtherComp :type "PrimitiveComponent Object Reference") (OtherBodyIndex :type Integer) (bFromSweep :type Boolean) (SweepResult :type "HitResult Structure (by ref)"))
  (bind _spawnpoint (`self.SpawnPoint`))
  (bind _spawnid (`self.SpawnID`))
  (if (== OtherActor (`GameplayStatics.GetPlayerCharacter` 0))
    (bind _gm_ref (message `/Game/Main/Blueprints/Data/Interfaces/Mode/BPI_GMMain.F_GameplayMode` (`GameplayStatics.GetGameMode`)))
    (if (`/Game/Main/Blueprints/Data/DataAssets/General/EditorSetting/PDA_DebugGame.ShouldSpawnEnemyByGate` (`/Game/Main/Blueprints/Data/Mode/GM_Gameplay.DT_EditorSetting` _gm_ref))
      (`/Engine/EditorBlueprintResources/StandardMacros.DoOnce` false :!label _label
        (:`Completed`
          (if (not (`KismetArrayLibrary.Array_IsEmpty` (`self.SpawnPoint`)))
            (`|ExecutionSequence`
              (:`then_0`
                (for _index (range (+ (`KismetArrayLibrary.Array_LastIndex` _spawnpoint) 1))
                  (bind _currentenemy (message `/Game/Main/Blueprints/Data/Interfaces/Mode/BPI_GMMain.IF_SpawnEnemy` (`GameplayStatics.GetGameMode`) (`|GetArrayItem` _spawnpoint _index) _spawnid))
                  (message `/Game/Marketplace/ALS/Blueprints/Interfaces/Enemy_BPI.IE_SetEnemyState` _currentenemy (`self.Enemy Type`))
                  (message `/Game/Main/Blueprints/Data/System/ObjectPooling/BP/Interface/BPI_Pooling.IE_SetSpawnID` _currentenemy _spawnid)))
              (:`then_1`
                (`/Engine/EditorBlueprintResources/StandardMacros.DoOnce` false :!label _label_2
                  (:`Completed`
                    (`self.F_DeactiveOtherGate`)))))))))))

(event `ResetCollision`
  (`self.SetActorEnableCollision` true)
  (goto _label :!via `Reset`))

(event `ResetCollisionOther`
  (goto _label_2 :!via `Reset`))

(event `DeactiveActiveGateOther`
  (`self.SetActorEnableCollision` false))

(event `SpawnpointSpawner`
  (bind (_returnvalue_location _returnvalue_rotation) (`KismetMathLibrary.BreakTransform` (`self.GetTransform`)))
  (bind _number_of_spawnpoint (`self.Number of SpawnPoint`))
  (if (> _number_of_spawnpoint 0)
    (`self.Despawn_SpawnCollection`)
    (for _ (range 1 (+ _number_of_spawnpoint 1))
      (bind _returnvalue (`|SpawnActorFromClass` "/Game/Main/Blueprints/Extra/Spawn/Enemy/BP_SpawnPoints.BP_SpawnPoints_C" (`KismetMathLibrary.MakeTransform` _returnvalue_location _returnvalue_rotation) "Undefined" "MultiplyWithRoot" null null))
      (`KismetArrayLibrary.Array_AddUnique` (`self.SpawnPoint`) _returnvalue)
      (`self.K2_AttachToActor` _returnvalue self "None" "KeepWorld" "KeepWorld" "KeepWorld" true))))

(event `Despawn_SpawnCollection`
  (bind _spawnpoint (`self.SpawnPoint`))
  (if (not (`KismetArrayLibrary.Array_IsEmpty` (`self.SpawnPoint`)))
    (for _array_element _spawnpoint
      (`self.K2_DestroyActor` _array_element))
    (`KismetArrayLibrary.Array_Clear` _spawnpoint)))

(fn `F_DeactiveOtherGate`
  (bind _gaterefother (`self.GateRefOther`))
  (if (`KismetArrayLibrary.Array_IsNotEmpty` _gaterefother)
    (for _array_element _gaterefother
      (`/Engine/EditorBlueprintResources/StandardMacros.IsValid` _array_element
        (:`Is Valid`
          (`self.DeactiveActiveGateOther` _array_element))))))

(fn `UserConstructionScript`)