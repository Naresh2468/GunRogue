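; BP_ActorActivation_BaseAI is an actor activation Blueprint that switches a list of target actors, presumably AI enemies, on or off.
; Activate calls the parent logic, then sends the activation interface message to every valid entry in TargetActor.
; One second after BeginPlay it calls Activate with false, so the targets start deactivated.
; A second, disconnected loop that deactivates the targets never runs.
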(event `self.ReceiveBeginPlay`
  (`KismetSystemLibrary.Delay` 1.0)
  (`self.Activate` false))

(event `self.Activate`
  (params (IsActivate :type Boolean))
  (`parent.Activate` IsActivate)
  (for _array_element (`self.TargetActor`)
    (`/Engine/EditorBlueprintResources/StandardMacros.IsValid` _array_element
      (:`Is Valid`
        (message `/Game/Marketplace/ALS/Blueprints/Interfaces/Enemy_BPI.IE_Activation` _array_element IsActivate)))))

(fn `UserConstructionScript`
  (`parent.UserConstructionScript`))