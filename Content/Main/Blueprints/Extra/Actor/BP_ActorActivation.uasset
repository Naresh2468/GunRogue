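; BP_ActorActivation is an actor that tracks an activation flag driven by the player character's overlap with its BCEntry component.
; Both begin and end overlap call ToggleActivate, which passes the inverse of IsActivate to Activate.
; Activate only stores the new value, as its debug print is disabled and no other logic reacts to the flag here.
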(event `self.BC - Entry.OnComponentBeginOverlap`
  (params (OverlappedComponent :type "PrimitiveComponent Object Reference") (OtherActor :type "Actor Object Reference") (OtherComp :type "PrimitiveComponent Object Reference") (OtherBodyIndex :type Integer) (bFromSweep :type Boolean) (SweepResult :type "HitResult Structure (by ref)"))
  (if (== OtherActor (`GameplayStatics.GetPlayerCharacter` 0))
    (`self.ToggleActivate`)))

(event `self.BC - Entry.OnComponentEndOverlap`
  (params (OverlappedComponent :type "PrimitiveComponent Object Reference") (OtherActor :type "Actor Object Reference") (OtherComp :type "PrimitiveComponent Object Reference") (OtherBodyIndex :type Integer))
  (if (== OtherActor (`GameplayStatics.GetPlayerCharacter` 0))
    (`self.ToggleActivate`)))

(event `ToggleActivate`
  (if (not (`self.Is Activate`))
    (`self.Activate` true)
    (else
      (`self.Activate` false))))

(event `Activate`
  (params (IsActivate :type Boolean))
  ; OtherLogic
  (bind _output_get (set `self.Is Activate` IsActivate))
  (`KismetSystemLibrary.PrintString` (`KismetStringLibrary.Conv_BoolToString` _output_get) :!enabledstate Disabled))

(fn `UserConstructionScript`)