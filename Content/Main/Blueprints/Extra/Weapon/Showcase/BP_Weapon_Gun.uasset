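; Showcase actor that displays a selected weapon's mesh and can spin it.
; An activation event toggles the RotatingMovement component's tick to start or stop the rotation.
; A weapon display event unhides the static mesh, lazily caches every weapon DataTable row into an array on first use, then applies the matching entry's mesh and scale by weapon name.
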(event `/Game/Main/Blueprints/Data/Interfaces/Weapon/WeaponUpdgrade/BPI_WeaponDisplay.IE_ShowCaseActive`
  (params (Activate :type Boolean))
  (`ActorComponent.SetComponentTickEnabled` (`self.RotatingMovement`) Activate))

(event `/Game/Main/Blueprints/Data/Interfaces/Weapon/WeaponUpdgrade/BPI_WeaponDisplay.IE_CurrentWeaponDisplay`
  (params (Weapon :type Name))
  (bind _staticmesh (`self.StaticMesh`))
  (`SceneComponent.SetHiddenInGame` (`self.StaticMesh`) false false)
  (if (not (`KismetArrayLibrary.Array_IsNotEmpty` (`self.WeaponDisplay`)))
    (`self.F_WeaponDisplayData`))
  (for _array_element (`self.WeaponDisplay`)
    (bind (_weaponname _weaponmesh _weapontransform) (break `/Game/Main/Blueprints/Data/Struct/Upgrade/S_WeaponDisplay` _array_element))
    (if (== _weaponname Weapon)
      (`StaticMeshComponent.SetStaticMesh` _staticmesh _weaponmesh)
      (`SceneComponent.SetRelativeScale3D` _staticmesh (.scale _weapontransform))
      (break))))

(fn `F_WeaponDisplayData`
  (bind _weapontable (`self.WeaponTable`))
  (bind _outrownames (`DataTableFunctionLibrary.GetDataTableRowNames` _weapontable))
  (for _array_element _outrownames
    (bind _returnvalue (`|GetDataTableRow` _weapontable _array_element)
      (:`then`
        (`KismetArrayLibrary.Array_Add` (`self.WeaponDisplay`) _returnvalue)))))

(fn `UserConstructionScript`)