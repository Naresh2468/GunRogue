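; BP_MissionCall is a trigger actor in the testing tool folder that signals mission stage changes to the game mode.
; When the player character overlaps its interaction detection component, it disables its collision, with no logic to re-enable it.
; It then switches on its MissionStage variable to send a mission start, hold time, resume or end message to the game mode.
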(event `self.BC - InteractDetection.OnComponentBeginOverlap`
  (params (OverlappedComponent :type "PrimitiveComponent Object Reference") (OtherActor :type "Actor Object Reference") (OtherComp :type "PrimitiveComponent Object Reference") (OtherBodyIndex :type Integer) (bFromSweep :type Boolean) (SweepResult :type "HitResult Structure (by ref)"))
  (bind _returnvalue (`GameplayStatics.GetGameMode`))
  (if (== OtherActor (`GameplayStatics.GetPlayerCharacter` 0))
    (`self.SetActorEnableCollision` false)
    (switch `/Game/Main/Blueprints/Data/Enum/Mission/E_MissionStats` (`self.MissionStage`)
      (:`NewEnumerator0`
        (message `/Game/Main/Blueprints/Data/Interfaces/Mode/BPI_GMMain.IE_MissionStart` _returnvalue))
      (:`NewEnumerator1`
        (message `/Game/Main/Blueprints/Data/Interfaces/Mode/BPI_GMMain.IE_CurrentHoldTime` _returnvalue true))
      (:`NewEnumerator3`
        (message `/Game/Main/Blueprints/Data/Interfaces/Mode/BPI_GMMain.IE_CurrentHoldTime` _returnvalue false))
      (:`NewEnumerator2`
        (message `/Game/Main/Blueprints/Data/Interfaces/Mode/BPI_GMMain.IE_MissionEnd` _returnvalue)))))

(fn `UserConstructionScript`)