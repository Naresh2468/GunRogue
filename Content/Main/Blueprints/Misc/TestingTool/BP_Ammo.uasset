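; BP_Ammo is a Blueprint in the testing tool folder that spawns ammo for the current gun.
; IECurrentAmmo looks up the gun's row in the AmmoData table and requests that ammo class from the GameMode's actor pool at the given transform.
; On success it marks the pooled actor in use, forwards the gun, transform and motion controller to it, and has the GameMode play haptic feedback.
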(event `/Game/Main/Blueprints/Data/Interfaces/Weapon/Ammo/BPI_AmmoPick.IE_CurrentAmmo`
  (params (CurrentGun :type Name) (AmmoSpawnTransform :type "Transform Structure") (MotionController :type "MotionControllerComponent Object Reference"))
  (bind _returnvalue (`|GetDataTableRow` (`self.AmmoData`) CurrentGun)
    (:`then`
      (bind (_ammoname _ammoclass) (break `/Game/Main/Blueprints/Data/Struct/Weapon/Ammo/S_AmmoInfo` _returnvalue))
      (`KismetSystemLibrary.PrintString` (`KismetStringLibrary.Conv_NameToString` _ammoname) :!enabledstate Disabled)
      (bind (_actorcall _issuccess) (message `/Game/Main/Blueprints/Data/Interfaces/Mode/BPI_GMMain.F_SpawnActorFromPool` (`GameplayStatics.GetGameMode`) _ammoclass AmmoSpawnTransform))
      (if _issuccess
        (message `/Game/Main/Blueprints/Data/System/ObjectPooling/BP/Interface/BPI_Pooling.IE_SetInuse` _actorcall true)
        ;[0.02083 0.02083 0.02083 0.5] Haptic Effects
        (message `/Game/Main/Blueprints/Data/Interfaces/Weapon/Ammo/BPI_AmmoPick.IE_CurrentAmmo` _actorcall CurrentGun AmmoSpawnTransform MotionController)
        (message `/Game/Main/Blueprints/Data/Interfaces/Mode/BPI_GMMain.IE_HapticEffect` (`GameplayStatics.GetGameMode`) MotionController "NewEnumerator0")))
    (:`RowNotFound`
      (`KismetSystemLibrary.PrintString` "Failed To Find Current Ammo Data" :!enabledstate Disabled))))

(fn `UserConstructionScript`)