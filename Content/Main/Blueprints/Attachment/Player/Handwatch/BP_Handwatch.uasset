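; VR handwatch attached to the player, with a health widget and a pause menu panel toggled through interface events.
; Toggling flips the GameMode's pause state and plays a timeline that scales, lifts and spins the panel in or out.
; The player pawn's right WidgetInteractionComponent drives a Niagara laser and cursor, shown only over hit-testable widgets.
; References to the pawn's widget interaction and aim motion controller components are cached on BeginPlay.
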(event `/Game/Main/Blueprints/Data/Interfaces/Attachment/PlayerHandwatch/BPI_HandWatchData.IE_LaserUpdate`
  (`self.Laser`))

(event `Laser`
  (`self.F_UpdateLaserAndCursor` (`self.Ray - Right`) (`self.WidgetInteractionRef - Right`) (`self.NS_RightLaser`) (`self.Cursor - Right`)))

(event `self.ReceiveBeginPlay`
  (`self.SetWidgetInteractionReferences`)
  (`self.SetMotionControllerReference`)
  (`self.F_LaserCursorVisibility` false (`self.NS_RightLaser`) (`self.Cursor - Right`)))

(event `/Game/Main/Blueprints/Data/Interfaces/Attachment/PlayerHandwatch/BPI_HandWatchData.IE_UpdateHealth`
  (message `/Game/Main/Blueprints/Data/Interfaces/UMG/PlayerStats/BPI_Playerstats.IE_UpdateHealth` (`WidgetComponent.GetWidget` (`self.W_PlayerHealth`))))

(event `/Game/Main/Blueprints/Data/Interfaces/Attachment/PlayerHandwatch/BPI_HandWatchData.IE_TogglePauseMenu`
  (bind _returnvalue (`GameplayStatics.GetGameMode`))
  (bind _gamepaused (message `/Game/Main/Blueprints/Data/Interfaces/Mode/BPI_GMMain.IF_PauseGameStatus` _returnvalue))
  (bind _returnvalue_2 (not _gamepaused))
  (`self.SmoothScaling` _returnvalue_2)
  (message `/Game/Main/Blueprints/Data/Interfaces/Mode/BPI_GMMain.IE_PauseGame` _returnvalue _returnvalue_2)
  (`self.F_UpdateLaserAndCursor` false (`self.WidgetInteractionRef - Right`) (`self.NS_RightLaser`) (`self.Cursor - Right`)))

(event `SmoothScaling`
  (params (ToggleVisible :type Boolean))
  (bind _panel (`self.Panel`))
  (bind (_relativelocation_x _relativelocation_y) (`KismetMathLibrary.BreakVector` (`SceneComponent.RelativeLocation` _panel)))
  (if ToggleVisible
    (bind (_direction _smooth) (`Timeline|Visiblity` :!via `PlayFromStart` :!label _label)
      (:`Update`
        (`SceneComponent.SetRelativeScale3D` _panel (`KismetMathLibrary.VLerp` (0.0 0.0 0.0) (`self.Relative Scale 3D`) _smooth))
        (`SceneComponent.K2_SetRelativeLocationAndRotation` _panel (`KismetMathLibrary.MakeVector` _relativelocation_x _relativelocation_y (`KismetMathLibrary.Lerp` 0.0 20.0 _smooth)) (`KismetMathLibrary.MakeRotator` 0.0 0.0 (`KismetMathLibrary.Lerp` 360.0 10.0 _smooth)) false false)))
    (else
      (goto _label :!via `ReverseFromEnd`))))

(fn `F_GetWidgetLocation`
  (params (Target :type "WidgetInteractionComponent Object Reference"))
  (returns (`Return Value Impact Point` :type "Vector Structure"))
  (bind (_returnvalue_bblockinghit _returnvalue_binitialoverlap _returnvalue_time _returnvalue_distance _returnvalue_location _returnvalue_impactpoint) (`GameplayStatics.BreakHitResult` (`WidgetInteractionComponent.GetLastHitResult` Target)))
  (return _returnvalue_impactpoint))

(fn `F_LaserCursorVisibility`
  (params (isVisible :type Boolean) (`Current Laser` :type "NiagaraComponent Object Reference") (`Current Cursor` :type "StaticMeshComponent Object Reference"))
  (bind _isvisible (`local.isVisible`))
  (`SceneComponent.SetVisibility` (`local.Current Laser`) _isvisible false)
  (`SceneComponent.SetVisibility` (`local.Current Cursor`) _isvisible false))

(fn `F_UpdateLaserAndCursor`
  (params (LaserAlwaysVisible :type Boolean) (`WIC - Main` :type "WidgetInteractionComponent Object Reference") (MainLaser :type "NiagaraComponent Object Reference") (MainCursor :type "StaticMeshComponent Object Reference"))
  (bind _mainlaser (`local.MainLaser`))
  ;[0 0 0] Check all necessary Condition
  (if (`KismetSystemLibrary.IsValid` `WIC - Main`)
    (if (and LaserAlwaysVisible (`WidgetInteractionComponent.IsOverHitTestVisibleWidget` (`local.WIC - Main`)))
      ;[0 0 0] Visible/Hide Toggle for cursor and Laser
      (`self.F_LaserCursorVisibility` true (`local.MainLaser`) (`local.MainCursor`))
      ;[0 0 0] Hit Result Calculate the point to set start and end point for laser beam and cursor endpoint for assign position on widget
      (set `self.LaserStartPoint` (`SceneComponent.K2_GetComponentLocation` (`local.WIC - Main`)))
      (if (`WidgetInteractionComponent.IsOverHitTestVisibleWidget` (`local.WIC - Main`))
        (bind _output_get (set `self.LaserEndPoint` (`self.F_GetWidgetLocation` (`local.WIC - Main`))))
        (`SceneComponent.K2_SetWorldLocation` (`local.MainCursor`) _output_get false false)
        (else
          (set `self.LaserEndPoint` (`self.F_WidgetEndLastPoint` (`local.WIC - Main`)))
          (`self.F_LaserCursorVisibility` false (`local.MainLaser`) (`local.MainCursor`))))
      (`NiagaraDataInterfaceArrayFunctionLibrary.SetNiagaraArrayVectorValue` _mainlaser "User.PointArray" 0 (`self.LaserStartPoint`))
      (`NiagaraDataInterfaceArrayFunctionLibrary.SetNiagaraArrayVectorValue` _mainlaser "User.PointArray" 1 (`self.LaserEndPoint`))
      (else
        (`self.F_LaserCursorVisibility` false (`local.MainLaser`) (`local.MainCursor`))))))

(fn `F_WidgetEndLastPoint`
  (params (`Current WidgetInteraction` :type "WidgetInteractionComponent Object Reference"))
  (returns (Endpoint :type "Vector Structure"))
  (return (+ (* (`SceneComponent.GetForwardVector` `Current WidgetInteraction`) (`WidgetInteractionComponent.InteractionDistance` `Current WidgetInteraction`)) (`self.LaserStartPoint`))))

(fn `GetWidgetInteractionComponent`
  (params (bRightWIC :type Boolean))
  (returns (ReturnValue :type "WidgetInteractionComponent Object Reference"))
  (return (select `bool` bRightWIC :`false` (`self.WidgetInteractionRef - Left`) :`true` (`self.WidgetInteractionRef - Right`))))

(fn `SetMotionControllerReference`
  (locals (LocalMotionControllers :type "Array of MotionControllerComponent Object Reference"))
  (bind _returnvalue (`GameplayStatics.GetPlayerPawn` 0))
  (bind _returnvalue_2 (`self.K2_GetComponentsByClass` _returnvalue "/Script/HeadMountedDisplay.MotionControllerComponent"))
  (`/Engine/EditorBlueprintResources/StandardMacros.IsValid` _returnvalue
    (:`Is Valid`
      (for _ (range 3)
        (if (> (`KismetArrayLibrary.Array_Length` _returnvalue_2) 0)
          (bind _output_get (set `local.LocalMotionControllers` _returnvalue_2))
          (for _array_element _output_get
            (if (== (`MotionControllerComponent.MotionSource` _array_element) (select `bool` (`self.bActiveMenuHandRight`) :`false` "LeftAim" :`true` "RightAim" :!type "Name"))
              (set `self.MotionControllerAimRef` _array_element))))))))

(fn `SetWidgetInteractionReferences`
  (locals (LocalWidgetInteractionComponents :type "Array of WidgetInteractionComponent Object Reference"))
  (bind _returnvalue (`GameplayStatics.GetPlayerPawn` 0))
  (bind _returnvalue_2 (`self.K2_GetComponentsByClass` _returnvalue "/Script/UMG.WidgetInteractionComponent"))
  (`/Engine/EditorBlueprintResources/StandardMacros.IsValid` _returnvalue
    (:`Is Valid`
      (if (> (`KismetArrayLibrary.Array_Length` _returnvalue_2) 0)
        (bind _output_get (set `local.LocalWidgetInteractionComponents` _returnvalue_2))
        (for _array_element _output_get
          (if (== (`WidgetInteractionComponent.PointerIndex` _array_element) 0)
            (set `self.WidgetInteractionRef - Left` _array_element)
            (else
              (set `self.WidgetInteractionRef - Right` _array_element))))))))

(fn `UserConstructionScript`)