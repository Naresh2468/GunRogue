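; BP_Holster is a player attachment that stores one tagged item, such as a weapon.
; A collision sphere tracks the overlapping candidate and shows the sphere mesh as an indicator while the holster is free.
; Holster and unholster events snap the candidate to the mesh's Holster socket, or detach the stored weapon and re-enable its physics.
; IsOccupied is set before the candidate validity check, so an empty holster call still marks it occupied.
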(event `self.Collision_Sphere.OnComponentBeginOverlap`
  (params (OverlappedComponent :type "PrimitiveComponent Object Reference") (OtherActor :type "Actor Object Reference") (OtherComp :type "PrimitiveComponent Object Reference") (OtherBodyIndex :type Integer) (bFromSweep :type Boolean) (SweepResult :type "HitResult Structure (by ref)"))
  (if (`self.ActorHasTag` OtherActor (`self.TagToCheck`))
    (set `self.HolsteredItem` OtherActor)
    (if (not (`self.IsOccupied?`))
      (`SceneComponent.SetVisibility` (`self.SM_Sphere`) true false))))

(event `/Game/Main/Blueprints/Data/Interfaces/Attachment/Holster/BPI_Holster.IE_Holster`
  (`self.HolsterWeapon`))

(event `/Game/Main/Blueprints/Data/Interfaces/Attachment/Holster/BPI_Holster.IE_Unholster`
  (`self.UnHolsterWeapon`))

(event `self.Collision_Sphere.OnComponentEndOverlap`
  (params (OverlappedComponent :type "PrimitiveComponent Object Reference") (OtherActor :type "Actor Object Reference") (OtherComp :type "PrimitiveComponent Object Reference") (OtherBodyIndex :type Integer))
  (if (== OtherActor (`self.HolsteredItem`))
    (set `self.HolsteredItem` null)
    (if (not (`self.IsOccupied?`))
      (`SceneComponent.SetVisibility` (`self.SM_Sphere`) false false))))

(fn `F_GetCurrentHolsteredItem`
  (returns (HolsteredItem :type "Actor Object Reference") (HolsterRef :type "/Game/Main/Blueprints/Attachment/Player/BP_Holster Object Reference"))
  (return (`self.HolsteredItem`) self))

(fn `HolsterWeapon`
  (bind _holstereditem (`self.HolsteredItem`))
  (if (not (`self.IsOccupied?`))
    (set `self.IsOccupied?` true)
    (`/Engine/EditorBlueprintResources/StandardMacros.IsValid` _holstereditem
      (:`Is Valid`
        (set `self.StoredWeapon` _holstereditem)
        (`self.K2_DetachFromActor` _holstereditem "KeepWorld" "KeepWorld" "KeepWorld")
        (`self.K2_AttachToComponent` _holstereditem (`self.SM_Sphere`) "Holster" "SnapToTarget" "SnapToTarget" "KeepWorld" true)
        (set `self.HolsteredItem` null)
        (`SceneComponent.SetVisibility` (`self.SM_Sphere`) true false)))))

(fn `UnHolsterWeapon`
  (bind _storedweapon (`self.StoredWeapon`))
  (set `self.IsOccupied?` false)
  (`/Engine/EditorBlueprintResources/StandardMacros.IsValid` _storedweapon
    (:`Is Valid`
      (`SceneComponent.SetVisibility` (`self.SM_Sphere`) false false)
      (`self.K2_DetachFromActor` _storedweapon "KeepWorld" "KeepWorld" "KeepWorld")
      (bind _currentweapon (message `/Game/Main/Blueprints/Data/Interfaces/Weapon/BPI_WeaponInterface.F_WeaponRef` _storedweapon))
      (`PrimitiveComponent.SetSimulatePhysics` (`/Game/Main/Blueprints/Weapons/BP_WeaponBase.WeaponMesh` _currentweapon) true)
      (set `self.TempStoredWeapon` _storedweapon)
      (set `self.StoredWeapon` null))))

(fn `UserConstructionScript`)