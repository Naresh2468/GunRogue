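; Gameplay GameMode for a VR hostage-rescue shooter, acting as the interface hub for mission flow, audio, stats, haptics and pause.
; Interface calls forward to pooling, timer, stats and audio components, while GameState broadcasts pause and reset.
; Enemies spawn from the pool, with reassignment as fallback.
; Rescues meeting the level table's hostage count (tutorial ends separately) trigger saving time and currency and unlocking the next level and reward weapon through GameInstance.
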(event `self.ReceiveBeginPlay`
  (`self.AudioDataFetch`))

(event `/Game/Main/Blueprints/Data/Interfaces/Mode/BPI_GMMain.IE_ReturnToPool`
  (params (Actor :type "Actor Object Reference"))
  ; Notify when the inital pooling completed
  (`/Game/Main/Blueprints/Data/System/ObjectPooling/BP/AC_Poolling.ResetActor` (`self.AC_Poolling`) Actor))

(event `MissionReward`
  (bind _returnvalue (`GameplayStatics.GetGameInstance`))
  ; Missison Reward
  (`self.F_UnlockLevel`)
  (`self.F_SaveGameContent`)
  (bind _level (message `/Game/Main/Blueprints/Data/Interfaces/Instance/BPI_GameInstance.F_CurrentLevel` (`GameplayStatics.GetGameInstance`)))
  (bind _returnvalue_2 (`|GetDataTableRow` "/Game/Main/Blueprints/Data/Table/Level/DT_Level.DT_Level" (`.Name_10_F74FA3AA4C3BD12409A81194C3A5B4CB` (break `/Game/Main/Blueprints/Data/Struct/LevelData/S_LevelProgression` _level)))
    (:`then`
      (bind (_gameplaydata _weaponupgrade) (message `/Game/Main/Blueprints/Data/Interfaces/SaveGame/BPI_SaveGame.IE_FetchData` _returnvalue))
      (for (_array_element _array_index) _weaponupgrade
        (if (`self.M_UnlockWeaponValidation` _array_element (`.Rewarded_11_6C45DFA541D294776C5F4BA53F009045` (break `/Game/Main/Blueprints/Data/Struct/LevelData/S_LevelInfo` _returnvalue_2)))
          (bind _structout (setmembers `/Game/Main/Blueprints/Data/Struct/Upgrade/S_UpgradeInformation` :`StructRef` _array_element :`Weapon Unlocked` true))
          (`KismetArrayLibrary.Array_Set` _weaponupgrade _array_index _structout)
          (message `/Game/Main/Blueprints/Data/Interfaces/SaveGame/BPI_SaveGame.IE_SaveWeaponDataGame` _returnvalue false _weaponupgrade)
          (break))))))

(event `/Game/Main/Blueprints/Data/Interfaces/Mode/BPI_GMMain.IE_MissionStart`
  ; Mission Call
  (`/Game/Main/Blueprints/Data/System/Time/AC_TimerSystem.StartTime` (`self.AC_TimerSystem`)))

(event `/Game/Main/Blueprints/Data/Interfaces/Tutorial/BPI_Tutorial.IE_TutorialEnd`
  ;[0.005208 0.005208 0.005208 0.5] Tutorial Section
  (`self.F_TutorialProgressSaved`)
  (`self.MissionReward`)
  (`self.MissionCompleted`)
  (`/Game/Main/Blueprints/Data/System/AudioManager/BPC_AudioManager.F_PlaySFX` (`self.BPC_AudioManager`) "NewEnumerator4" "GameEnd" true (`self.K2_GetActorLocation` (`GameplayStatics.GetPlayerCharacter` 0))))

(event `/Game/Main/Blueprints/Data/Interfaces/Tutorial/BPI_Tutorial.IE_TutorialSkip`
  ;[0.005208 0.005208 0.005208 0.5] Tutorial Section
  (`self.F_TutorialProgressSaved`)
  (`self.MissionReward`))

(event `MissionCompleted`
  ; After all the conditon of mission meet then that time Call
  (message `/Game/Marketplace/ALS/Blueprints/Interfaces/BPI_Player.IE_MissionCompleted` (`GameplayStatics.GetPlayerCharacter` 0)))

(event `/Game/Main/Blueprints/Data/Interfaces/Mode/BPI_GMMain.IE_CurrentHoldTime`
  (params (Activate :type Boolean))
  ; Hold Time
  (`/Game/Main/Blueprints/Data/System/Time/AC_TimerSystem.F_TimerPauseController` (`self.AC_TimerSystem`) Activate))

(event `/Game/Main/Blueprints/Data/Interfaces/Mode/BPI_GMMain.IE_MissionEnd`
  ; Mission Call
  (`self.F_SaveGameContent`))

(event `/Game/Main/Blueprints/Data/Interfaces/Mode/BPI_GMMain.IE_RestartGame`
  ; After all the conditon of mission meet then that time Call
  (message `/Game/Marketplace/ALS/Blueprints/Interfaces/BPI_Player.IE_PlayerRestartPauseGame` (`GameplayStatics.GetPlayerCharacter` 0))
  (`self.F_BackgroundMusic`))

(event `/Game/Main/Blueprints/Data/Interfaces/Mode/BPI_GMMain.IE_PauseGame`
  (params (GamePaused :type Boolean))
  (bind _output_get (set `self.Game Paused` GamePaused))
  (`self.F_PausedActor` _output_get))

(event `/Game/Main/Blueprints/Data/Interfaces/Mode/BPI_GMMain.IE_MissionFailedRestartGame`
  ; Mission Call
  (message `/Game/Marketplace/ALS/Blueprints/Interfaces/BPI_Player.IE_MissionFailedPlayerRestart` (`GameplayStatics.GetPlayerCharacter` 0)))

(event `/Game/Main/Blueprints/Data/Interfaces/Mode/BPI_GMMain.IE_HapticEffect`
  (params (MotionController :type "MotionControllerComponent Object Reference") (Haptic :type "/Game/Main/Blueprints/Data/Enum/Haptic/E_HapticEffect Enum" :default "NewEnumerator0"))
  (`PlayerController.PlayHapticEffect` (`GameplayStatics.GetPlayerController` 0) (select `byte` Haptic :`0` (`self.HP_Defaut`) :`1` (`self.HP_Short`) :`2` (`self.HP_LowIntense`)) (`self.F_HandHeld` MotionController) 1.0 false))

(event `/Game/Main/Blueprints/Data/Interfaces/Mode/BPI_GMMain.IE_ResetGameElement`
  ; this call by the Player
  (message `/Game/Main/Blueprints/Data/Interfaces/EventManager/BPI_Events.IE_Publish_ResetGameElement` (`GameplayStatics.GetGameState`)))

(event `/Game/Main/Blueprints/Data/System/AudioManager/SoundData/Interface/BPI_Audio.IE_SetMasterVolume`
  (params (Volume :type "Float (double-precision)"))
  ; AudioManager
  (`/Game/Main/Blueprints/Data/System/AudioManager/BPC_AudioManager.F_SetMasterVolume` (`self.BPC_AudioManager`) Volume))

(event `/Game/Main/Blueprints/Data/System/AudioManager/SoundData/Interface/BPI_Audio.IE_PlayBGMSound`
  (params (`Audio-Type` :type "/Game/Main/Blueprints/Data/System/AudioManager/SoundData/Enums/E_BGM Enum" :default "NewEnumerator0") (AudioName :type Name))
  ; AudioManager
  (`/Game/Main/Blueprints/Data/System/AudioManager/BPC_AudioManager.F Play BGM` (`self.BPC_AudioManager`) `Audio-Type` AudioName))

(event `/Game/Main/Blueprints/Data/System/AudioManager/SoundData/Interface/BPI_Audio.IE_SetBGMVolume`
  (params (Volume :type "Float (double-precision)"))
  ; AudioManager
  (`/Game/Main/Blueprints/Data/System/AudioManager/BPC_AudioManager.F Set BGM Volume` (`self.BPC_AudioManager`) Volume))

(event `/Game/Main/Blueprints/Data/System/AudioManager/SoundData/Interface/BPI_Audio.IE_PlaySFXSound`
  (params (`Audio-Type` :type "/Game/Main/Blueprints/Data/System/AudioManager/SoundData/Enums/E_SFX Enum" :default "NewEnumerator1") (AudioName :type Name) (PlaySound2D :type Boolean) (Location :type "Vector Structure"))
  ; AudioManager
  (`/Game/Main/Blueprints/Data/System/AudioManager/BPC_AudioManager.F_PlaySFX` (`self.BPC_AudioManager`) `Audio-Type` AudioName PlaySound2D Location))

(event `/Game/Main/Blueprints/Data/System/AudioManager/SoundData/Interface/BPI_Audio.IE_SetSFXVolume`
  (params (Volume :type "Float (double-precision)"))
  ; AudioManager
  (`/Game/Main/Blueprints/Data/System/AudioManager/BPC_AudioManager.F Set SFX Volume` (`self.BPC_AudioManager`) Volume))

(event `/Game/Main/Blueprints/Data/System/AudioManager/SoundData/Interface/BPI_Audio.IE_SetUIVolume`
  (params (Volume :type "Float (double-precision)"))
  ; AudioManager
  (`/Game/Main/Blueprints/Data/System/AudioManager/BPC_AudioManager.F Set UI Volume` (`self.BPC_AudioManager`) Volume))

(event `/Game/Main/Blueprints/Data/Interfaces/Gameplay/BPI_GameStats.IE_TotalHitTaken`
  ; Frequently update
  (`/Game/Main/Blueprints/Data/Component/BPC_Stats.F_TotalHitTaken` (`self.BPC_Stats`)))

(event `/Game/Main/Blueprints/Data/Interfaces/Gameplay/BPI_GameStats.IE_HeadShot`
  ; Frequently update
  (`/Game/Main/Blueprints/Data/Component/BPC_Stats.F_HeadShots` (`self.BPC_Stats`)))

(event `/Game/Main/Blueprints/Data/Interfaces/Gameplay/BPI_GameStats.IE_TotalKill`
  ; Frequently update
  (`/Game/Main/Blueprints/Data/Component/BPC_Stats.F_TotalKill` (`self.BPC_Stats`)))

(event `/Game/Main/Blueprints/Data/Interfaces/Gameplay/BPI_GameStats.IE_SuspectNeutralized`
  ; Frequently update
  (`/Game/Main/Blueprints/Data/Component/BPC_Stats.F_TotalRescue` (`self.BPC_Stats`))
  (`self.F_MissionCompleted`))

(event `/Game/Main/Blueprints/Data/Interfaces/Gameplay/BPI_GameStats.IE_GameCompletedTime`
  ; After mission completed then it will update
  (`/Game/Main/Blueprints/Data/Component/BPC_Stats.F_MissionCompleteTime` :`self` (`self.BPC_Stats`)))

(event `/Game/Main/Blueprints/Data/Interfaces/Gameplay/BPI_GameStats.IE_Accuracy_Hit`
  ; After mission completed then it will update
  (`/Game/Main/Blueprints/Data/Component/BPC_Stats.F_CurrentHitCount` (`self.BPC_Stats`)))

(event `/Game/Main/Blueprints/Data/Interfaces/Gameplay/BPI_GameStats.IE_Accuracy_Fire`
  ; After mission completed then it will update
  (`/Game/Main/Blueprints/Data/Component/BPC_Stats.F_CurrentFireCount` (`self.BPC_Stats`)))

(fn `AudioDataFetch`
  (bind (_gameplaydata _weaponupgrade _gamesetting) (message `/Game/Main/Blueprints/Data/Interfaces/SaveGame/BPI_SaveGame.IE_FetchData` (`GameplayStatics.GetGameInstance`)))
  (bind ((`AudioMaster_67_B6BDF19245C5738FAB24B289489DF69B` _audiomaster) (`AudioMusic_69_02D7995E4AB56837625569AC2A3B03ED` _audiomusic) (`AudioSFX_71_C00D5B3F4FAF5864D0059CA42584C604` _audiosfx)) (break `/Game/Main/Blueprints/Data/Struct/GameStats/S_GameSetting` _gamesetting))
  (`/Game/Main/Blueprints/Data/System/AudioManager/BPC_AudioManager.F_SetGlobalAudioVolume` (`self.BPC_AudioManager`) _audiomaster _audiomusic _audiosfx))

(fn `F_BackgroundMusic`
  (bind _bpc_audiomanager (`self.BPC_AudioManager`))
  (bind _bpc_audiomanager_2 (`self.BPC_AudioManager`))
  (bind _level (message `/Game/Main/Blueprints/Data/Interfaces/Instance/BPI_GameInstance.F_CurrentLevel` (`GameplayStatics.GetGameInstance`)))
  (switch `name` (`.Name_10_F74FA3AA4C3BD12409A81194C3A5B4CB` (break `/Game/Main/Blueprints/Data/Struct/LevelData/S_LevelProgression` _level))
    (:`MainMenu`
      (`/Game/Main/Blueprints/Data/System/AudioManager/BPC_AudioManager.F Play BGM` _bpc_audiomanager "NewEnumerator0" "Music - MainMenu"))
    (:`Tutorial`
      (`/Game/Main/Blueprints/Data/System/AudioManager/BPC_AudioManager.F Play BGM` _bpc_audiomanager "NewEnumerator0" "Music - Tutorial")
      (`/Game/Main/Blueprints/Data/System/AudioManager/BPC_AudioManager.F_PlaySFX` (`self.BPC_AudioManager`) "NewEnumerator4" "GameStart" true (`self.K2_GetActorLocation` (`GameplayStatics.GetPlayerCharacter` 0)) :!label _label))
    (:`Restro`
      (`/Game/Main/Blueprints/Data/System/AudioManager/BPC_AudioManager.F Play BGM` _bpc_audiomanager_2 "NewEnumerator0" "Music - Restaurant")
      (goto _label))
    (:`Factory`
      (`/Game/Main/Blueprints/Data/System/AudioManager/BPC_AudioManager.F Play BGM` _bpc_audiomanager_2 "NewEnumerator0" "Music - Factory")
      (goto _label))
    (:`House`
      (`/Game/Main/Blueprints/Data/System/AudioManager/BPC_AudioManager.F Play BGM` _bpc_audiomanager_2 "NewEnumerator0" "Music - House")
      (goto _label))))

(fn `F_CurrentWeaponUpgradeData`
  (params (WeaponIndex :type Integer))
  (returns (`S Current Weapon Upgrade` :type "/Game/Main/Blueprints/Data/Struct/Upgrade/S_UpgradeInformation Structure"))
  (bind _returnvalue (`|GetDataTableRow` (`self.CurrentWeaponData`) (`|GetArrayItem` (`self.WeaponRowNames`) WeaponIndex))
    (:`then`
      (return _returnvalue))
    (:`RowNotFound`
      (return))))

(fn `F_GameplayMode`
  (returns (GM_Ref :type "/Game/Main/Blueprints/Data/Mode/GM_Gameplay Object Reference"))
  (return self))

(fn `F_GetAllWeaponData`
  (for _array_element (`self.WeaponRowNames`)
    (bind _returnvalue (`|GetDataTableRow` (`self.CurrentWeaponData`) _array_element)
      (:`then`
        (`KismetArrayLibrary.Array_Add` (`self.AllWeaponData`) _returnvalue)))))

(fn `F_GetBGMVolume`
  (returns (Value :type "Float (double-precision)"))
  (return (`/Game/Main/Blueprints/Data/System/AudioManager/BPC_AudioManager.BGM_Volume` (`self.BPC_AudioManager`))))

(fn `F_GetMasterVolume`
  (returns (Value :type "Float (double-precision)"))
  (return (`/Game/Main/Blueprints/Data/System/AudioManager/BPC_AudioManager.Master_Volume` (`self.BPC_AudioManager`))))

(fn `F_GetMusicDuration`
  (returns (Duration :type "Float (double-precision)"))
  (return (`/Game/Main/Blueprints/Data/System/AudioManager/BPC_AudioManager.MusicDuration` (`self.BPC_AudioManager`))))

(fn `F_GetSFXDuration`
  (returns (Duration :type "Float (double-precision)"))
  (return (`/Game/Main/Blueprints/Data/System/AudioManager/BPC_AudioManager.SFXDuration` (`self.BPC_AudioManager`))))

(fn `F_GetSfxVolume`
  (returns (Value :type "Float (double-precision)"))
  (return (`/Game/Main/Blueprints/Data/System/AudioManager/BPC_AudioManager.SFX_Volume` (`self.BPC_AudioManager`))))

(fn `F_HandHeld`
  (params (Target :type "MotionControllerComponent Object Reference"))
  (returns (ReturnValue :type "EControllerHand Enum"))
  (`/Engine/EditorBlueprintResources/StandardMacros.IsValid` Target
    (:`Is Valid`
      (return (select `bool` (== (`MotionControllerComponent.MotionSource` Target) "LeftGrip") :`false` "Right" :`true` "Left" :!type "EControllerHand Enum")))))

(fn `F_MissionCompleteChecking`
  (returns (MissionCompleted :type Boolean))
  ; Checking the Level Completion for checking the number of Hostage recuse based on level
  (bind _level (message `/Game/Main/Blueprints/Data/Interfaces/Instance/BPI_GameInstance.F_CurrentLevel` (`GameplayStatics.GetGameInstance`)))
  (bind _returnvalue (`|GetDataTableRow` (`self.DT_Level Data`) (`.Name_10_F74FA3AA4C3BD12409A81194C3A5B4CB` (break `/Game/Main/Blueprints/Data/Struct/LevelData/S_LevelProgression` _level)))
    (:`then`
      (return (>= (`/Game/Main/Blueprints/Data/Component/BPC_Stats.TotalHostageRescue` (`self.BPC_Stats`)) (`.Hostage_2_0D119A89426BA485A9AEE7B3FE27BA33` (break `/Game/Main/Blueprints/Data/Struct/Mission/S_Mission` (`.MissionData_15_2BB7326848CB6F3EA023ABA4EA443C66` (break `/Game/Main/Blueprints/Data/Struct/LevelData/S_LevelInfo` _returnvalue)))))))
    (:`RowNotFound`
      (return false))))

(fn `F_MissionCompleted`
  (bind _completionresult (`self.IE_OnMissionCompletionValidation`))
  (bind _level (message `/Game/Main/Blueprints/Data/Interfaces/Instance/BPI_GameInstance.F_CurrentLevel` (`GameplayStatics.GetGameInstance`)))
  (if (and _completionresult (!= (`.Number_19_A68E959147C7259E5587A2AE4218D0A2` (break `/Game/Main/Blueprints/Data/Struct/LevelData/S_LevelProgression` _level)) 0))
    (`self.MissionReward`)
    (`self.MissionCompleted`)))

(fn `F_PausedActor`
  (params (PauseGame :type Boolean))
  (message `/Game/Main/Blueprints/Data/Interfaces/EventManager/BPI_Events.IE_Publish_PauseActor` (`GameplayStatics.GetGameState`) PauseGame))

(fn `F_SaveGameContent`
  (bind _returnvalue (`GameplayStatics.GetGameInstance`))
  (bind _ac_timersystem (`self.AC_TimerSystem`))
  (`/Game/Main/Blueprints/Data/System/AudioManager/BPC_AudioManager.F_PlaySFX` (`self.BPC_AudioManager`) "NewEnumerator4" "GameEnd" true (`self.K2_GetActorLocation` (`GameplayStatics.GetPlayerCharacter` 0)))
  (`/Game/Main/Blueprints/Data/System/Time/AC_TimerSystem.StopTimer` _ac_timersystem)
  (bind _tc_endtime (`/Game/Main/Blueprints/Data/System/Time/AC_TimerSystem.F_CurrentTime` _ac_timersystem))
  (`/Game/Main/Blueprints/Data/Component/BPC_Stats.F_MissionCompleteTime` (`self.BPC_Stats`) _tc_endtime)
  (bind _gameplaydata (message `/Game/Main/Blueprints/Data/Interfaces/SaveGame/BPI_SaveGame.IE_FetchData` _returnvalue))
  (bind _structout (setmembers `/Game/Main/Blueprints/Data/Struct/GameStats/S_Gameplay` :`StructRef` _gameplaydata :`TotalPlayTime` _tc_endtime :`ROECurrency` (+ (`.ROECurrency_38_B93094A047F4657E81F63B86A6E06404` (break `/Game/Main/Blueprints/Data/Struct/GameStats/S_Gameplay` _gameplaydata)) (`.MissionROEReward_32_4DDEE9194F085496C0C34D9737800EA2` (break `/Game/Main/Blueprints/Data/Struct/GameStats/S_GameStats` (`/Game/Main/Blueprints/Data/Component/BPC_Stats.MainStats` (`self.BPC_Stats`)))))))
  (message `/Game/Main/Blueprints/Data/Interfaces/SaveGame/BPI_SaveGame.IE_SaveGameplayGame` _returnvalue false _structout))

(fn `F_SpawnActorFromPool`
  (params (TargetActor :type "Actor Class Reference") (SpawnTransform :type "Transform Structure"))
  (returns (ActorCall :type "Actor Object Reference") (isSuccess :type Boolean))
  (bind _ac_poolling (`self.AC_Poolling`))
  (bind _storespawnactor (`/Game/Main/Blueprints/Data/System/ObjectPooling/BP/AC_Poolling.StoreSpawnActor` _ac_poolling))
  (`/Game/Main/Blueprints/Data/System/ObjectPooling/BP/AC_Poolling.CE_FindFirstActorAvailable` _ac_poolling TargetActor SpawnTransform)
  (return _storespawnactor (`KismetSystemLibrary.IsValid` _storespawnactor)))

(fn `F_SpawnEnemy`
  (params (Actor :type "Actor Object Reference") (SpawnID :type Name))
  (returns (Enemy :type "Actor Object Reference"))
  (bind (_returnvalue_location _returnvalue_rotation) (`KismetMathLibrary.BreakTransform` (`self.GetTransform` Actor)))
  (bind _returnvalue (`KismetMathLibrary.MakeTransform` _returnvalue_location _returnvalue_rotation))
  ; Enemy Spawn for Room Stage
  (`/Engine/EditorBlueprintResources/StandardMacros.IsValid` Actor
    (:`Is Valid`
      (bind (_actorcall _issuccess) (`self.F_SpawnActorFromPool` "/Game/Marketplace/ALS/Blueprints/CharacterLogic/BaseShootingEnemy_BP.BaseShootingEnemy_BP_C" _returnvalue))
      (if _issuccess
        (message `/Game/Main/Blueprints/Data/System/ObjectPooling/BP/Interface/BPI_Pooling.IE_SetInuse` _actorcall true)
        (return _actorcall)
        (else
          (bind (_assignedactorresult _assignedactor) (`/Game/Main/Blueprints/Data/System/ObjectPooling/BP/AC_Poolling.F_ReassignActor` (`self.AC_Poolling`) "/Game/Marketplace/ALS/Blueprints/CharacterLogic/BaseShootingEnemy_BP.BaseShootingEnemy_BP_C" _returnvalue SpawnID))
          (message `/Game/Main/Blueprints/Data/System/ObjectPooling/BP/Interface/BPI_Pooling.IE_SetInuse` _assignedactor true)
          (return _assignedactor))))))

(fn `F_TutorialProgressSaved`
  (bind _returnvalue (`GameplayStatics.GetGameInstance`))
  (bind _gameplaydata (message `/Game/Main/Blueprints/Data/Interfaces/SaveGame/BPI_SaveGame.IE_FetchData` _returnvalue))
  (if (not (`.isTutorialCompleted_40_5098B0AF458BBB86BBF673A0592929BF` (break `/Game/Main/Blueprints/Data/Struct/GameStats/S_Gameplay` _gameplaydata)))
    (bind _structout (setmembers `/Game/Main/Blueprints/Data/Struct/GameStats/S_Gameplay` :`StructRef` _gameplaydata :`isTutorialCompleted` true))
    (message `/Game/Main/Blueprints/Data/Interfaces/SaveGame/BPI_SaveGame.IE_SaveGameplayGame` _returnvalue false _structout)))

(fn `F_UnlockLevel`
  (bind _returnvalue (`GameplayStatics.GetGameInstance`))
  (bind _level (message `/Game/Main/Blueprints/Data/Interfaces/Instance/BPI_GameInstance.F_CurrentLevel` _returnvalue))
  (bind (_gameplaydata _weaponupgrade _gamesetting _leveldata) (message `/Game/Main/Blueprints/Data/Interfaces/SaveGame/BPI_SaveGame.IE_FetchData` _returnvalue))
  (setmembers `/Game/Main/Blueprints/Data/Struct/LevelData/S_LevelInfo` :`StructRef` (`|GetArrayItem` _leveldata (`KismetMathLibrary.Clamp` (+ (`.Number_19_A68E959147C7259E5587A2AE4218D0A2` (break `/Game/Main/Blueprints/Data/Struct/LevelData/S_LevelProgression` _level)) 1) 0 (`KismetArrayLibrary.Array_LastIndex` _leveldata))) :`Unlocked` true)
  (message `/Game/Main/Blueprints/Data/Interfaces/SaveGame/BPI_SaveGame.IE_SaveGameLevelData` _returnvalue false _leveldata))

(fn `F_WeaponUpgradeData`
  (bind _outrownames (`DataTableFunctionLibrary.GetDataTableRowNames` (`self.CurrentWeaponData`)))
  (bind _output_get (set `self.WeaponRowNames` _outrownames))
  (set `self.TotalWeapons` (`KismetArrayLibrary.Array_LastIndex` _output_get)))

(fn `IE_OnMissionCompletionValidation`
  (returns (CompletionResult :type Boolean))
  (bind _missioncompleted (`self.F_MissionCompleteChecking`))
  (return _missioncompleted))

(fn `IF_PauseGameStatus`
  (returns (GamePaused :type Boolean))
  (return (`self.Game Paused`)))

(fn `IF_SpawnEnemy`
  (params (SpawnTarget :type "Actor Object Reference") (SpawnID :type Name))
  (returns (CurrentEnemy :type "Actor Object Reference"))
  (bind _enemy (`self.F_SpawnEnemy` SpawnTarget SpawnID))
  (return _enemy))

(fn `UserConstructionScript`)