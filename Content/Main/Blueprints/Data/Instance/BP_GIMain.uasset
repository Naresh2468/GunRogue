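; Main game instance that owns the SG_Main save object and loads or creates it on Init.
; A new save is seeded with default gameplay and settings values plus weapon and level rows from data tables.
; Interface events write each data section and save synchronously or asynchronously behind DoOnce guards, while IEFetchData returns all sections.
; It also tracks current level, forwards volume changes to the game mode and computes total playtime.
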(event `self.ReceiveInit`
  ;[0 0 0 0.5] Save Game
  (`self.IE_MainLoadGame` false (`self.GameSlotName`)))

(event `/Game/Main/Blueprints/Data/Interfaces/SaveGame/BPI_SaveGame.IE_MainLoadGame`
  (params (Async :type Boolean) (SlotName :type String))
  ;[0 0 0 0.5] Save Game
  (bind _returnvalue (`GameplayStatics.DoesSaveGameExist` SlotName))
  (if _returnvalue
    (if Async
      (`/Engine/EditorBlueprintResources/StandardMacros.DoOnce` false :!label _label
        (:`Completed`
          (bind _savegame (`AsyncActionHandleSaveGame.AsyncLoadGameFromSlot` SlotName)
            (:`Completed`
              (`self.Ref_SaveGame`
                (:`then`
                  _)
                (:`else`
                  (bind _assg_main (cast `/Game/Main/Blueprints/Data/System/SaveGame/SG_Main` _savegame))
                  (set `self.Ref_SaveGame` _assg_main)))
              (`self.ED_OnGameLoad`)
              (goto _label :!via `Reset`)))))
      (else
        (bind _returnvalue_2 (`GameplayStatics.LoadGameFromSlot` SlotName))
        (`self.Ref_SaveGame`
          (:`then`)
          (:`else`
            (bind _assg_main_2 (cast `/Game/Main/Blueprints/Data/System/SaveGame/SG_Main` _returnvalue_2))
            (set `self.Ref_SaveGame` _assg_main_2)))))
    (else
      (bind _returnvalue_3 (`GameplayStatics.CreateSaveGameObject` "/Game/Main/Blueprints/Data/System/SaveGame/SG_Main.SG_Main_C"))
      (set `self.Ref_SaveGame` _returnvalue_3)
      (`self.F_InitialGameSaving`))))

(event `/Game/Main/Blueprints/Data/Interfaces/SaveGame/BPI_SaveGame.IE_MainSaveGame`
  (params (Aysnc :type Boolean) (SlotName :type String))
  (bind _ref_savegame (`self.Ref_SaveGame`))
  ;[0 0 0 0.5] Save Game
  (if Aysnc
    (`/Engine/EditorBlueprintResources/StandardMacros.DoOnce` false :!label _label_2
      (:`Completed`
        (`AsyncActionHandleSaveGame.AsyncSaveGameToSlot` _ref_savegame SlotName
          (:`Completed`
            (goto _label_2 :!via `Reset`)))))
    (else
      (`GameplayStatics.SaveGameToSlot` _ref_savegame SlotName))))

(event `/Game/Main/Blueprints/Data/Interfaces/SaveGame/BPI_SaveGame.IE_SaveGameplayGame`
  (params (Async :type Boolean) (Gameplay :type "/Game/Main/Blueprints/Data/Struct/GameStats/S_Gameplay Structure"))
  ;[0 0 0 0.5] Save Game
  (set `/Game/Main/Blueprints/Data/System/SaveGame/SG_Main.S Gameplay` Gameplay (`self.Ref_SaveGame`))
  (`self.IE_MainSaveGame` Async (`self.GameSlotName`)))

(event `/Game/Main/Blueprints/Data/Interfaces/SaveGame/BPI_SaveGame.IE_SaveWeaponDataGame`
  (params (Async :type Boolean) (WeaponData :type "Array of /Game/Main/Blueprints/Data/Struct/Upgrade/S_UpgradeInformation Structure (by ref)"))
  ;[0 0 0 0.5] Save Game
  (set `/Game/Main/Blueprints/Data/System/SaveGame/SG_Main.S Weapon` WeaponData (`self.Ref_SaveGame`))
  (`self.IE_MainSaveGame` Async (`self.GameSlotName`)))

(event `/Game/Main/Blueprints/Data/Interfaces/SaveGame/BPI_SaveGame.IE_SaveGameSetting`
  (params (Async :type Boolean) (Gameplay :type "/Game/Main/Blueprints/Data/Struct/GameStats/S_GameSetting Structure"))
  ;[0 0 0 0.5] Save Game
  (set `/Game/Main/Blueprints/Data/System/SaveGame/SG_Main.S GameSetting` Gameplay (`self.Ref_SaveGame`))
  (`self.IE_MainSaveGame` Async (`self.GameSlotName`)))

(event `/Game/Main/Blueprints/Data/Interfaces/SaveGame/BPI_SaveGame.IE_SaveGameLevelData`
  (params (Async :type Boolean) (Level :type "Array of /Game/Main/Blueprints/Data/Struct/LevelData/S_LevelInfo Structure (by ref)"))
  ;[0 0 0 0.5] Save Game
  (set `/Game/Main/Blueprints/Data/System/SaveGame/SG_Main.S LevelData` Level (`self.Ref_SaveGame`))
  (`self.IE_MainSaveGame` Async (`self.GameSlotName`)))

(event `/Game/Main/Blueprints/Data/Interfaces/Instance/BPI_GameInstance.IE_LevelDetail`
  (params (LevelNumber :type "/Game/Main/Blueprints/Data/Struct/LevelData/S_LevelProgression Structure"))
  ;[0 0 0 0.5] Save Game
  (set `self.CurrentLevelProgress` LevelNumber))

(event `/Game/Main/Blueprints/Data/Interfaces/Instance/BPI_GameInstance.IE_MasterVolume`
  (params (Volume :type "Float (double-precision)"))
  ;[0.02604 0.02604 0.02604 0.5] AudioSetup
  (message `/Game/Main/Blueprints/Data/System/AudioManager/SoundData/Interface/BPI_Audio.IE_SetMasterVolume` (`GameplayStatics.GetGameMode`) Volume))

(event `/Game/Main/Blueprints/Data/Interfaces/Instance/BPI_GameInstance.IE_MusicVolume`
  (params (Volume :type "Float (double-precision)"))
  ;[0.02604 0.02604 0.02604 0.5] AudioSetup
  (message `/Game/Main/Blueprints/Data/Interfaces/Instance/BPI_GameInstance.IE_MusicVolume` (`GameplayStatics.GetGameMode`) Volume))

(event `/Game/Main/Blueprints/Data/Interfaces/Instance/BPI_GameInstance.IE_BGMVolume`
  (params (Volume :type "Float (double-precision)"))
  ;[0.02604 0.02604 0.02604 0.5] AudioSetup
  (message `/Game/Main/Blueprints/Data/System/AudioManager/SoundData/Interface/BPI_Audio.IE_SetBGMVolume` (`GameplayStatics.GetGameMode`) Volume))

(event `/Game/Main/Blueprints/Data/Interfaces/Instance/BPI_GameInstance.IE_SFXVolume`
  (params (Volume :type "Float (double-precision)"))
  ;[0.02604 0.02604 0.02604 0.5] AudioSetup
  (message `/Game/Main/Blueprints/Data/System/AudioManager/SoundData/Interface/BPI_Audio.IE_SetSFXVolume` (`GameplayStatics.GetGameMode`) Volume))

(fn `F_CurrentLevel`
  (returns (Level :type "/Game/Main/Blueprints/Data/Struct/LevelData/S_LevelProgression Structure"))
  (return (`self.CurrentLevelProgress`)))

(fn `F_CurrentTime`
  (returns (CurrentTime :type "Timecode Structure (by ref)"))
  (bind _output_get (set `self.Current Time` (+ (`self.F_PreviousTime`) (`GameplayStatics.GetTimeSeconds`))))
  (bind _structout (setmembers `Timecode` :`StructRef` (`self.M_SecondsToTimeCode` _output_get)))
  (return _structout))

(fn `F_GetAllLevelData`
  (returns (Level :type "Array of /Game/Main/Blueprints/Data/Struct/LevelData/S_LevelInfo Structure"))
  (locals (AllLevelData :type "Array of /Game/Main/Blueprints/Data/Struct/LevelData/S_LevelInfo Structure"))
  (bind _currentleveldata (`self.CurrentLevelData`))
  (bind _outrownames (`DataTableFunctionLibrary.GetDataTableRowNames` _currentleveldata))
  (for _array_element _outrownames
    (bind _returnvalue (`|GetDataTableRow` _currentleveldata _array_element)
      (:`then`
        (`KismetArrayLibrary.Array_Add` (`local.AllLevelData`) _returnvalue))))
  (return (`local.AllLevelData`)))

(fn `F_GetAllWeaponData`
  (returns (Weapon :type "Array of /Game/Main/Blueprints/Data/Struct/Upgrade/S_UpgradeInformation Structure"))
  (locals (AllWeaponData :type "Array of /Game/Main/Blueprints/Data/Struct/Upgrade/S_UpgradeInformation Structure"))
  (bind _outrownames (`DataTableFunctionLibrary.GetDataTableRowNames` (`self.CurrentWeaponData`)))
  (for _array_element _outrownames
    (bind _returnvalue (`|GetDataTableRow` (`self.CurrentWeaponData`) _array_element)
      (:`then`
        (`KismetArrayLibrary.Array_Add` (`local.AllWeaponData`) _returnvalue))))
  (return (`local.AllWeaponData`)))

(fn `F_GIRef`
  (returns (GIRef :type "/Game/Main/Blueprints/Data/Instance/BP_GIMain Object Reference"))
  (return self))

(fn `F_InitialGameSaving`
  (`self.IE_SaveGameplayGame` false (make `/Game/Main/Blueprints/Data/Struct/GameStats/S_Gameplay` (struct) 200))
  (`self.IE_SaveGameSetting` false (make `/Game/Main/Blueprints/Data/Struct/GameStats/S_GameSetting` 0 true true 1 1 1 1 1 1 1 1.0 0.5 1.0))
  (bind _weapon (`self.F_GetAllWeaponData`))
  (`self.IE_SaveWeaponDataGame` false _weapon)
  (bind _level (`self.F_GetAllLevelData`))
  (`self.IE_SaveGameLevelData` false _level))

(fn `F_PreviousTime`
  (returns (PreviousTotalTime :type "Float (double-precision)"))
  (return (`self.M_TimeCodeToSeconds` (`self.TC_TotalPlaytime`))))

(fn `IE_FetchData`
  (returns (GameplayData :type "/Game/Main/Blueprints/Data/Struct/GameStats/S_Gameplay Structure") (WeaponUpgrade :type "Array of /Game/Main/Blueprints/Data/Struct/Upgrade/S_UpgradeInformation Structure") (GameSetting :type "/Game/Main/Blueprints/Data/Struct/GameStats/S_GameSetting Structure") (LevelData :type "Array of /Game/Main/Blueprints/Data/Struct/LevelData/S_LevelInfo Structure"))
  (bind _ref_savegame (`self.Ref_SaveGame`))
  (return (`/Game/Main/Blueprints/Data/System/SaveGame/SG_Main.S Gameplay` _ref_savegame) (`/Game/Main/Blueprints/Data/System/SaveGame/SG_Main.S Weapon` _ref_savegame) (`/Game/Main/Blueprints/Data/System/SaveGame/SG_Main.S GameSetting` _ref_savegame) (`/Game/Main/Blueprints/Data/System/SaveGame/SG_Main.S LevelData` _ref_savegame)))