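; BPC_Stats is a component that records mission statistics: kills, headshots, hits taken, hostage rescues, completion time and shooting accuracy.
; Simple functions increment or set members of the MainStats struct, while bullets fired and hit are counted in separate variables.
; F_CurrentData recomputes accuracy as hits divided by shots fired, then returns the struct.
; The rescue count is stored in the SuspectRescue member and mirrored to TotalHostageRescue.
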(fn `F_Accuracy`
  (params (Hit :type Integer) (Fire :type Integer))
  (setmembers `/Game/Main/Blueprints/Data/Struct/GameStats/S_GameStats` :`StructRef` (`self.MainStats`) :`TotalAccuracy` (/ Hit Fire)))

(fn `F_CurrentData`
  (returns (MainStats :type "/Game/Main/Blueprints/Data/Struct/GameStats/S_GameStats Structure"))
  (`self.F_Accuracy` (`self.CurrentBulletHitCount`) (`self.CurrentBulletFireCount`))
  (return (`self.MainStats`)))

(fn `F_CurrentFireCount`
  (`/Engine/EditorBlueprintResources/StandardMacros.IncrementInt` (`self.CurrentBulletFireCount`)))

(fn `F_CurrentHitCount`
  (`/Engine/EditorBlueprintResources/StandardMacros.IncrementInt` (`self.CurrentBulletHitCount`)))

(fn `F_HeadShots`
  (bind _mainstats (`self.MainStats`))
  (bind _result (`/Engine/EditorBlueprintResources/StandardMacros.IncrementInt` (`.TotalHeadShot_4_67A88BC5408E163E9659E7BB9DAE0CF2` (break `/Game/Main/Blueprints/Data/Struct/GameStats/S_GameStats` _mainstats)))
    (:`  `
      (setmembers `/Game/Main/Blueprints/Data/Struct/GameStats/S_GameStats` :`StructRef` _mainstats :`TotalHeadShot` _result))))

(fn `F_MissionCompleteTime`
  (params (CurrentTime :type "Timecode Structure"))
  (setmembers `/Game/Main/Blueprints/Data/Struct/GameStats/S_GameStats` :`StructRef` (`self.MainStats`) :`MissionCompletedTime` CurrentTime))

(fn `F_TotalHitTaken`
  (bind _mainstats (`self.MainStats`))
  (bind _result (`/Engine/EditorBlueprintResources/StandardMacros.IncrementInt` (`.TotalHitTaken_21_10DB2C9541620B33038D1A9D75BE928A` (break `/Game/Main/Blueprints/Data/Struct/GameStats/S_GameStats` _mainstats)))
    (:`  `
      (setmembers `/Game/Main/Blueprints/Data/Struct/GameStats/S_GameStats` :`StructRef` _mainstats :`TotalHitTaken` _result))))

(fn `F_TotalKill`
  (bind _mainstats (`self.MainStats`))
  (bind _result (`/Engine/EditorBlueprintResources/StandardMacros.IncrementInt` (`.TotalKills_5_63C64CD84493D5D0CE96308E259F1D03` (break `/Game/Main/Blueprints/Data/Struct/GameStats/S_GameStats` _mainstats)))
    (:`  `
      (setmembers `/Game/Main/Blueprints/Data/Struct/GameStats/S_GameStats` :`StructRef` _mainstats :`TotalKills` _result))))

(fn `F_TotalRescue`
  (bind _mainstats (`self.MainStats`))
  (bind _result (`/Engine/EditorBlueprintResources/StandardMacros.IncrementInt` (`.SuspectRescue_10_746DA8C54366888AE2A2C799E3722701` (break `/Game/Main/Blueprints/Data/Struct/GameStats/S_GameStats` _mainstats)))
    (:`  `
      (bind _output_get (set `self.TotalHostageRescue` _result))
      (setmembers `/Game/Main/Blueprints/Data/Struct/GameStats/S_GameStats` :`StructRef` _mainstats :`Suspect Rescue` _result))))