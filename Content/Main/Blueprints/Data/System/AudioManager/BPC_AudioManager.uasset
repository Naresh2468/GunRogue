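; Audio manager component that plays music, SFX and UI sounds by category and name, and controls their volumes.
; Each play function finds its clip in a per-type DataTable, using the category enum as row name.
; Music reuses one player-attached component, 2D SFX restart a shared one, and positional SFX and UI are one-shots.
; Volume setters override Sound Mix classes by index for master, music (capped at 0.8), SFX and UI.
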(fn `F Play BGM`
  (params (`Music Type` :type "/Game/Main/Blueprints/Data/System/AudioManager/SoundData/Enums/E_BGM Enum" :default "NewEnumerator0") (`Audio Name` :type Name :default "Sound Name"))
  (bind _audioclip (`self.F_SetCurrentAudio` "NewEnumerator0" (`|GetEnumeratorNameAsString` `Music Type`) `Audio Name`))
  (`self.AC_BGM`
    (:`then`
      (`AudioComponent.SetSound` (`self.AC_BGM`) _audioclip))
    (:`else`
      (bind _player (message `/Game/Marketplace/ALS/Blueprints/Interfaces/Player_BPI.F_PlayerRef` (`GameplayStatics.GetPlayerCharacter` 0)))
      (bind _mesh (`Character.Mesh` _player))
      (bind _returnvalue (`GameplayStatics.SpawnSoundAttached` _audioclip _mesh "None" (`SceneComponent.K2_GetComponentLocation` _mesh) (struct) "KeepWorldPosition" false 1.0 1.0 0.0 "/Game/Main/Blueprints/Data/System/AudioManager/SoundData/Class/Attutention/SA_Bgm.SA_Bgm" null false))
      (bind _output_get (set `self.AC_BGM` _returnvalue))))
  (`AudioComponent.Play` _output_get 0.1)
  (set `self.MusicDuration` (`SoundBase.Duration` _audioclip)))

(fn `F Set BGM Volume`
  (params (BGMVolume :type "Float (double-precision)"))
  (bind _output_get (set `self.BGM_Volume` BGMVolume))
  (`self.F_SetMainVolumeData` 1 (`KismetMathLibrary.MapRangeClamped` _output_get 0.0 1.0 0.0 0.8)))

(fn `F Set SFX Volume`
  (params (SFXVolume :type "Float (double-precision)"))
  (bind _output_get (set `self.SFX_Volume` SFXVolume))
  (`self.F_SetMainVolumeData` 2 _output_get))

(fn `F Set UI Volume`
  (params (`UI Volume` :type "Float (single-precision)"))
  (bind _output_get (set `self.UI_Volume` `UI Volume`))
  (`self.F_SetMainVolumeData` 3 _output_get))

(fn `F_GetMusicDuration`
  (returns (NewParam :type "Float (double-precision)"))
  (return (`self.MusicDuration`)))

(fn `F_GetSFXDuration`
  (returns (NewParam :type "Float (double-precision)"))
  (return (`self.SFXDuration`)))

(fn `F_PlaySFX`
  (params (`SFX Type` :type "/Game/Main/Blueprints/Data/System/AudioManager/SoundData/Enums/E_SFX Enum" :default "NewEnumerator1") (`Audio Name` :type Name :default "Sound Name") (PlaySound2D :type Boolean) (Location :type "Vector Structure"))
  (bind _audioclip (`self.F_SetCurrentAudio` "NewEnumerator1" (`|GetEnumeratorNameAsString` `SFX Type`) `Audio Name`))
  (if PlaySound2D
    (`self.SFXSoundController`
      (:`then`
        (`AudioComponent.SetSound` (`self.SFXSoundController`) _audioclip)
        (set `self.SFXDuration` (`SoundBase.Duration` _audioclip)))
      (:`else`
        (`/Engine/EditorBlueprintResources/StandardMacros.IsValid` _audioclip
          (:`Is Valid`
            (bind _returnvalue (`GameplayStatics.SpawnSound2D` _audioclip 1.0 1.0 0.0 null))
            (set `self.SFXSoundController` _returnvalue)))))
    (`AudioComponent.Stop` (`self.SFXSoundController`))
    (`AudioComponent.Play` (`self.SFXSoundController`) 0.0)
    (else
      (`GameplayStatics.PlaySoundAtLocation` _audioclip (`local.Location`) (struct) 1.0 1.0 0.0 "/Game/Main/Blueprints/Data/System/AudioManager/SoundData/Class/Attutention/SA_DefaultGame.SA_DefaultGame" null null null)
      (`/Engine/EditorBlueprintResources/StandardMacros.IsValid` _audioclip
        (:`Is Valid`
          (set `self.SFXDuration` (`SoundBase.Duration` _audioclip)))))))

(fn `F_PlayUI`
  (params (`UI Type` :type "/Game/Main/Blueprints/Data/System/AudioManager/SoundData/Enums/E_UI Enum" :default "NewEnumerator0") (`Audio Name` :type Name :default "Sound Name"))
  (bind _audioclip (`self.F_SetCurrentAudio` "NewEnumerator2" (`|GetEnumeratorNameAsString` `UI Type`) `Audio Name`))
  (`GameplayStatics.PlaySound2D` _audioclip 1.0 1.0 0.0 null null))

(fn `F_SetCurrentAudio`
  (params (`Audio-Type` :type "/Game/Main/Blueprints/Data/System/AudioManager/SoundData/Enums/E_AudioType Enum" :default "NewEnumerator5") (`Sub-Type` :type String) (`Audio Name` :type Name))
  (returns (AudioClip :type "SoundBase Object Reference"))
  (locals (bISAudioClipFound :type Boolean))
  ;[0.01562 0.01562 0.01562] Fetch the data table by the current audio Type of main and after the audio use the sub type of audio Category for table element.
  (set `local.bISAudioClipFound` false)
  (bind (_out_bgm _out_sfx _out_ui) (`self.F_SetDataTable` (`local.Audio-Type`) (`KismetStringLibrary.Conv_StringToName` (`local.Sub-Type`))))
  ;[0.005208 0.005208 0.005208] After main sub type of audio check the audio of each element and if the valid then audio play
  (for _array_element (select `/Game/Main/Blueprints/Data/System/AudioManager/SoundData/Enums/E_AudioType` (`local.Audio-Type`) :`NewEnumerator0` (`.SoundBase_26_62DBDFFB4A9F5A5E01A4FA90E8209B2F` (break `/Game/Main/Blueprints/Data/System/AudioManager/SoundData/Struct/BGM/S_BGM` _out_bgm)) :`NewEnumerator1` (`.SoundBase_27_62DBDFFB4A9F5A5E01A4FA90E8209B2F` (break `/Game/Main/Blueprints/Data/System/AudioManager/SoundData/Struct/BGM/S_SFX` _out_sfx)) :`NewEnumerator2` (`.SoundBase_27_62DBDFFB4A9F5A5E01A4FA90E8209B2F` (break `/Game/Main/Blueprints/Data/System/AudioManager/SoundData/Struct/BGM/S_UI` _out_ui)))
    (bind (_audioname _audioclip) (break `/Game/Main/Blueprints/Data/System/AudioManager/SoundData/Struct/General/S_AudioDetail` _array_element))
    (if (== `Audio Name` _audioname)
      ;;[0 0 0] Caution: - Make Sure the Audio is assign to the data table.
      (`|ExecutionSequence`
        (:`then_0`
          (`/Engine/EditorBlueprintResources/StandardMacros.IsValid` _audioclip
            (:`Is Valid`
              (set `local.bISAudioClipFound` true)
              (return _audioclip))))
        (:`then_1`
          (break)))))
  (if (not (`local.bISAudioClipFound`))
    (return null)))

(fn `F_SetDataTable`
  (params (CurrentType :type "/Game/Main/Blueprints/Data/System/AudioManager/SoundData/Enums/E_AudioType Enum" :default "NewEnumerator5") (CurrentRow :type Name))
  (returns (`Out BGM` :type "/Game/Main/Blueprints/Data/System/AudioManager/SoundData/Struct/BGM/S_BGM Structure") (`Out SFX` :type "/Game/Main/Blueprints/Data/System/AudioManager/SoundData/Struct/BGM/S_SFX Structure") (`Out UI` :type "/Game/Main/Blueprints/Data/System/AudioManager/SoundData/Struct/BGM/S_UI Structure"))
  (bind _currentrow (`local.CurrentRow`))
  (switch `/Game/Main/Blueprints/Data/System/AudioManager/SoundData/Enums/E_AudioType` CurrentType
    (:`NewEnumerator0`
      (bind _returnvalue (`|GetDataTableRow` (`self.DT_BGM`) (`local.CurrentRow`))
        (:`then`
          (return _returnvalue))))
    (:`NewEnumerator1`
      (bind _returnvalue_2 (`|GetDataTableRow` (`self.DT_SFX`) _currentrow)
        (:`then`
          (return (struct) _returnvalue_2))))
    (:`NewEnumerator2`
      (bind _returnvalue_3 (`|GetDataTableRow` (`self.DT_UI`) _currentrow)
        (:`then`
          (return (struct) (struct) _returnvalue_3))))))

(fn `F_SetGlobalAudioVolume`
  (params (BGMVolume :type "Float (double-precision)") (SFXVolume :type "Float (double-precision)") (`UI Volume` :type "Float (single-precision)"))
  (`self.F Set BGM Volume` BGMVolume)
  (`self.F Set SFX Volume` SFXVolume)
  (`self.F Set UI Volume` `UI Volume`))

(fn `F_SetMainVolumeData`
  (params (`SoundClass Index` :type Integer) (Volume :type "Float (single-precision)"))
  (bind ((`SoundClassObject` _soundclassobject) (`PitchAdjuster` _pitchadjuster)) (break `SoundClassAdjuster` (`|GetArrayItem` (`SoundMix.SoundClassEffects` (`self.AM - AudioController`)) `SoundClass Index`)))
  (`GameplayStatics.SetSoundMixClassOverride` (`self.AM - AudioController`) _soundclassobject Volume _pitchadjuster))

(fn `F_SetMasterVolume`
  (params (MasterVolume :type "Float (double-precision)"))
  (bind _output_get (set `self.Master_Volume` MasterVolume))
  (`self.F_SetMainVolumeData` 0 _output_get))