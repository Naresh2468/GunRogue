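; Actor component that pre-spawns and recycles pooled actors, when pooling is enabled in DADebug.
; From BeginPlay it walks numbered data table rows, spawning each class's quota in a grid offset from BP_SpawnPointElements, with delays between rows, then fires a completion dispatcher.
; Interface messages track class and in-use state, letting it hand out free actors, return them to default locations, or relocate busy ones with a different spawn ID.
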(event `self.ReceiveBeginPlay`
  (`self.PoolInitial`))

(event `PoolInitial`
  ;[0.01562 0.01562 0.01562] Pooling Concept
  (if (`/Game/Main/Blueprints/Data/DataAssets/General/EditorSetting/PDA_DebugGame.ShouldPool` (`self.DA_Debug`))
    (set `self.DataNumber` 1)
    (bind _returnvalue (`GameplayStatics.GetActorOfClass` "/Game/Main/Blueprints/Data/System/ObjectPooling/BP/BP_SpawnPointElements.BP_SpawnPointElements_C"))
    (`/Engine/EditorBlueprintResources/StandardMacros.IsValid` _returnvalue
      (:`Is Valid`
        (set `self.Spawn Transform Location` (`Actor.K2_GetActorLocation` _returnvalue))
        (`self.PoolProcess`)))))

(event `PoolProcess`
  ;[0.01562 0.01562 0.01562] Pooling Concept
  (bind (_actor _spawnlimit _actorlifetime _isvalid) (`self.F_GetActor` :!label _label))
  (if _isvalid
    (for _index (range 1 (+ (`KismetMathLibrary.Conv_ByteToInt` _spawnlimit) 1))
      (bind _returnvalue (+ (`self.Spawn Transform Location`) (`KismetMathLibrary.MakeVector` (* _index 100) (* (`self.DataNumber`) 40))))
      (bind _returnvalue_2 (`|SpawnActorFromClass` (`self.PoolActorClass`) (`KismetMathLibrary.MakeTransform` _returnvalue) "AdjustIfPossibleButAlwaysSpawn" "MultiplyWithRoot" null null))
      (`KismetArrayLibrary.Array_AddUnique` (`self.ActorPool`) _returnvalue_2)
      (message `/Game/Main/Blueprints/Data/System/ObjectPooling/BP/Interface/BPI_Pooling.IE_SetInfo` _returnvalue_2 (select `bool` (`self.DebugMode`) :`false` (`KismetMathLibrary.Conv_ByteToDouble` _actorlifetime) :`true` (`self.ActorTimeToALive`)) _returnvalue)
      (message `/Game/Main/Blueprints/Data/System/ObjectPooling/BP/Interface/BPI_Pooling.IE_SetInuse` _returnvalue_2 false))
    (`/Engine/EditorBlueprintResources/StandardMacros.IncrementInt` (`self.DataNumber`)
      (:`  `
        (`KismetSystemLibrary.Delay` 0.5)
        (`self.PoolRestActor`)))
    (else
      (`self.ED_PoolProcess`))))

(event `PoolRestActor`
  ;[0.01562 0.01562 0.01562] Pooling Concept
  (goto _label))

(event `CE_FindFirstActorAvailable`
  (params (TargetActor :type "Object Class Reference") (AssingLocation :type "Transform Structure"))
  ;[0.02604 0.02604 0.02604] InCase Not working in functionCall
  (set `self.StoreSpawnActor` null)
  (for _array_element (`self.ActorPool`)
    (bind _classref (message `/Game/Main/Blueprints/Data/System/ObjectPooling/BP/Interface/BPI_Pooling.F_GetClass` _array_element))
    (if (== _classref TargetActor)
      (bind _is_usedactor (message `/Game/Main/Blueprints/Data/System/ObjectPooling/BP/Interface/BPI_Pooling.F_GetData` _array_element))
      (if (not _is_usedactor)
        (`|ExecutionSequence`
          (:`then_0`
            (set `self.StoreSpawnActor` _array_element))
          (:`then_1`
            (break)))
        (else
          (`KismetSystemLibrary.PrintString` "Object in USE" true true (struct :`R` 1.0 :`G` 0.217517 :`A` 1.0) :!enabledstate Disabled)))))
  (`self.AssginActor` AssingLocation))

(event `AssginActor`
  (params (Transform :type "Transform Structure (by ref)"))
  (bind _storespawnactor (`self.StoreSpawnActor`))
  ;[0.02604 0.02604 0.02604] InCase Not working in functionCall
  (`/Engine/EditorBlueprintResources/StandardMacros.IsValid` _storespawnactor
    (:`Is Valid`
      (`Actor.K2_SetActorTransform` _storespawnactor Transform false true)
      (message `/Game/Main/Blueprints/Data/System/ObjectPooling/BP/Interface/BPI_Pooling.IE_SetInuse` _storespawnactor true))
    (:`Is Not Valid`
      (set `self.StoreSpawnActor` null))))

(event `ResetAllElement`
  ;[0.02604 0.02604 0.02604] InCase Not working in functionCall
  (for _array_element (`self.ActorPool`)
    (bind (_is_usedactor _defaultlocation) (message `/Game/Main/Blueprints/Data/System/ObjectPooling/BP/Interface/BPI_Pooling.F_GetData` _array_element))
    (if _is_usedactor
      (message `/Game/Main/Blueprints/Data/System/ObjectPooling/BP/Interface/BPI_Pooling.IE_SetInuse` _array_element false)
      (`Actor.K2_SetActorTransform` _array_element (`KismetMathLibrary.MakeTransform` _defaultlocation) false false))))

(event `ResetActor`
  (params (Actor :type "Actor Object Reference"))
  ;[0.02604 0.02604 0.02604] InCase Not working in functionCall
  (bind (_is_usedactor _defaultlocation) (message `/Game/Main/Blueprints/Data/System/ObjectPooling/BP/Interface/BPI_Pooling.F_GetData` Actor))
  (if _is_usedactor
    (message `/Game/Main/Blueprints/Data/System/ObjectPooling/BP/Interface/BPI_Pooling.IE_SetInuse` Actor false)
    (`Actor.K2_SetActorTransform` Actor (`KismetMathLibrary.MakeTransform` _defaultlocation) false false)))

(event `ReassignActorPosition`
  (params (Transform :type "Transform Structure (by ref)"))
  (bind _storespawnactor (`self.StoreSpawnActor`))
  (`/Engine/EditorBlueprintResources/StandardMacros.IsValid` _storespawnactor
    (:`Is Valid`
      (`Actor.K2_SetActorTransform` _storespawnactor (`KismetMathLibrary.MakeTransform` (.location Transform) (.rotation Transform)) false true))))

(fn `F_FindFirstActorAvailable`
  (params (TargetRef :type "Actor Class Reference"))
  (returns (PoolActorOut :type "Actor Object Reference"))
  (for _array_element (`self.ActorPool`)
    (bind _classref (message `/Game/Main/Blueprints/Data/System/ObjectPooling/BP/Interface/BPI_Pooling.F_GetClass` _array_element))
    (if (== _classref TargetRef)
      (bind _is_usedactor (message `/Game/Main/Blueprints/Data/System/ObjectPooling/BP/Interface/BPI_Pooling.F_GetData` _array_element))
      (if (not _is_usedactor)
        (return _array_element)))))

(fn `F_GetActor`
  (returns (Actor :type "Actor Class Reference") (SpawnLimit :type Byte) (ActorLifetime :type Byte) (IsValid :type Boolean))
  (bind _returnvalue (`|GetDataTableRow` (`self.MainData Table`) (`KismetStringLibrary.Conv_StringToName` (`KismetStringLibrary.Conv_IntToString` (`self.DataNumber`))))
    (:`then`
      (bind (_actorname _spawnactor _spawnlimit _actorlifetime) (break `/Game/Main/Blueprints/Data/System/ObjectPooling/Data/S_Actor` _returnvalue))
      (bind _output_get (set `self.PoolActorClass` _spawnactor))
      (return _output_get _spawnlimit _actorlifetime (`KismetSystemLibrary.IsValidClass` _output_get)))
    (:`RowNotFound`
      (set `self.PoolActorClass` null)
      (return null 0 0 false))))

(fn `F_PoolingProcess`)

(fn `F_ReassignActor`
  (params (`Spawn Actor` :type "Object Class Reference") (Transform :type "Transform Structure (by ref)") (SpawnID :type Name))
  (returns (AssignedActorResult :type Boolean) (AssignedActor :type "Actor Object Reference"))
  (set `self.StoreSpawnActor` null)
  (for _array_element (`self.ActorPool`)
    (bind _classref (message `/Game/Main/Blueprints/Data/System/ObjectPooling/BP/Interface/BPI_Pooling.F_GetClass` _array_element))
    (if (== _classref `Spawn Actor`)
      ; To avoid the same enemy reassign
      (bind _spawnid (message `/Game/Main/Blueprints/Data/System/ObjectPooling/BP/Interface/BPI_Pooling.IE_GetSpawnID` _array_element))
      (if (!= _spawnid SpawnID)
        (bind _is_usedactor (message `/Game/Main/Blueprints/Data/System/ObjectPooling/BP/Interface/BPI_Pooling.F_GetData` _array_element))
        (if _is_usedactor
          (bind _output_get (set `self.StoreSpawnActor` _array_element))
          (`self.ReassignActorPosition` Transform)
          (return (`KismetSystemLibrary.IsValid` _output_get) _output_get))))))

(fn `F_SpawnFromPool`
  (params (TargetActor :type "Actor Class Reference") (SpawnTransform :type "Transform Structure"))
  (returns (PooledActor :type "Actor Object Reference") (SuccessFull :type Boolean))
  (bind _poolactorout (`self.F_FindFirstActorAvailable` TargetActor))
  (`/Engine/EditorBlueprintResources/StandardMacros.IsValid` _poolactorout
    (:`Is Valid`
      (bind (_sweephitresult _returnvalue) (`Actor.K2_SetActorTransform` _poolactorout SpawnTransform false false))
      (message `/Game/Main/Blueprints/Data/System/ObjectPooling/BP/Interface/BPI_Pooling.IE_SetInuse` _poolactorout true)
      (return _poolactorout _returnvalue))
    (:`Is Not Valid`
      (`KismetSystemLibrary.PrintString` "Failed To Find Object" true true (struct :`R` 1.0 :`G` 0.041906 :`A` 1.0) :!enabledstate Disabled))))