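; Reusable cooldown actor component that runs a timed cooldown and broadcasts start, end and interrupt events through dispatchers.
; A single timer drives it, and modifying the time restarts that timer with either a new duration or the initial duration plus an offset.
; Tick runs only during cooldown, at an interval mapped from SmoothProgression, updating normalized and raw remaining time and printing a debug string.
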(event `self.ReceiveTick`
  (params (DeltaSeconds :type "Float (single-precision)"))
  (bind _cooldowntimer (`self.CooldownTimer`))
  (bind _returnvalue (`KismetSystemLibrary.K2_GetTimerRemainingTimeHandle` _cooldowntimer))
  (if (`KismetSystemLibrary.K2_IsValidTimerHandle` _cooldowntimer)
    (set `self.CooldownWaitTime` (`KismetMathLibrary.NormalizeToRange` _returnvalue 0.0 (+ (`KismetSystemLibrary.K2_GetTimerElapsedTimeHandle` _cooldowntimer) _returnvalue)))
    (bind _output_get (set `self.TimeRemaining` _returnvalue))
    (`KismetSystemLibrary.PrintString` (`KismetStringLibrary.Concat_StrStr` (`KismetSystemLibrary.GetDisplayName` (`self.GetOwner`)) ":" (`KismetStringLibrary.Conv_DoubleToString` _output_get)))))

(fn `F_CooldownInterrupt`
  (`self.F_EndCooldown`)
  (`self.ED_CooldownInterrupt`))

(fn `F_EndCooldown`
  (bind _cooldowntimer (`self.CooldownTimer`))
  (if (`KismetSystemLibrary.K2_IsValidTimerHandle` _cooldowntimer)
    (`self.SetComponentTickEnabled` false)
    (`KismetSystemLibrary.K2_ClearAndInvalidateTimerHandle` _cooldowntimer)
    (`self.ED_CooldownEnd`)))

(fn `F_ModificationCooldown`
  (params (CurrentCoolDownTime :type "Float (single-precision)"))
  (bind _cooldowntimer (`self.CooldownTimer`))
  (if (`KismetSystemLibrary.K2_IsValidTimerHandle` _cooldowntimer)
    (`KismetSystemLibrary.K2_ClearAndInvalidateTimerHandle` _cooldowntimer)
    (bind _returnvalue (`KismetSystemLibrary.K2_SetTimerDelegate` (`|CreateDelegate` :!event `F_EndCooldown`) CurrentCoolDownTime))
    (set `self.CooldownTimer` _returnvalue)))

(fn `F_ModifyCooldownTime`
  (params (ModifyCooldownTime :type "Float (double-precision)") (`Reset & ClearTime` :type Boolean))
  (`self.F_ModificationCooldown` (select `bool` `Reset & ClearTime` :`false` (+ (`self.InitialTime`) (`local.ModifyCooldownTime`)) :`true` ModifyCooldownTime :!type "Float (single-precision)")))

(fn `F_StartCooldown`
  (params (CurrentCooldownTime :type "Float (double-precision)"))
  (`self.SetComponentTickInterval` (`KismetMathLibrary.MapRangeClamped` (`self.SmoothProgression`) 0.0 1.0 0.06 0.2))
  (if (not (`KismetSystemLibrary.K2_IsValidTimerHandle` (`self.CooldownTimer`)))
    (set `self.InitialTime` CurrentCooldownTime)
    (set `self.CooldownWaitTime` 0.0)
    (bind _returnvalue (`KismetSystemLibrary.K2_SetTimerDelegate` (`|CreateDelegate` :!event `F_EndCooldown`) CurrentCooldownTime))
    (set `self.CooldownTimer` _returnvalue)
    (`self.SetComponentTickEnabled` true)
    (`self.ED_CooldownStart`)))