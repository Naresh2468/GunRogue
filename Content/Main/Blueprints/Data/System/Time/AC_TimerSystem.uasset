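; Timer component that runs a clock either counting up or counting down in hours, minutes and seconds.
; A looping one-second timer handle drives it, with support for start, stop, pause and reset.
; Count-up advances a Timecode struct, while countdown uses separate integers seeded from preset values and clears the timer at zero.
; Ticks fire the EDTimer dispatcher, which receives the Timecode only when counting up.
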(event `StartTime`
  ;[0.005208 0.005208 0.005208] Setup
  (`self.TimerModeConfig` true))

(event `TimerModeConfig`
  (params (TimerForward :type Boolean))
  ;[0.005208 0.005208 0.005208] Setup
  (`self.F_TimerControllerToggle` TimerForward))

(event `StopTimer`
  (bind _timer_controller (`self.Timer Controller`))
  ;[0.005208 0.005208 0.005208] Setup
  (if (`KismetSystemLibrary.K2_IsValidTimerHandle` _timer_controller)
    (`KismetSystemLibrary.K2_ClearAndInvalidateTimerHandle` _timer_controller)))

(fn `F_CurrentTime`
  (returns (TC_EndTime :type "Timecode Structure"))
  (return (`self.TC_Counter`)))

(fn `F_ForwardTimerCalculcation`
  (bind _tc_counter (`self.TC_Counter`))
  (bind _tc_counter_2 (`self.TC_Counter`))
  (bind _tc_counter_3 (`self.TC_Counter`))
  (if (>= (`.Seconds` (break `Timecode` _tc_counter_2)) 60)
    (set `self.Sec` 0)
    (setmembers `Timecode` :`StructRef` _tc_counter_2 :`Seconds` 0)
    (if (>= (`self.Min`) 60)
      (setmembers `Timecode` :`StructRef` _tc_counter_2 :`Minutes` 0)
      (bind _result (`/Engine/EditorBlueprintResources/StandardMacros.IncrementInt` (`.Hours` (break `Timecode` _tc_counter_2)))
        (:`  `
          (setmembers `Timecode` :`StructRef` _tc_counter_2 :`Hours` _result)))
      (else
        (bind _result_2 (`/Engine/EditorBlueprintResources/StandardMacros.IncrementInt` (`.Minutes` (break `Timecode` _tc_counter)))
          (:`  `
            (setmembers `Timecode` :`StructRef` _tc_counter :`Minutes` _result_2)))))
    (else
      (bind _result_3 (`/Engine/EditorBlueprintResources/StandardMacros.IncrementInt` (`.Seconds` (break `Timecode` _tc_counter_3)))
        (:`  `
          (setmembers `Timecode` :`StructRef` _tc_counter_3 :`Seconds` _result_3)))))
  (`self.ED_Timer` (`self.TC_Counter`)))

(fn `F_GetCurrentTime`
  (returns (Hour :type Byte) (Min :type Byte) (Sec :type Byte))
  (return (`self.Hour`) (`self.Min`) (`self.Sec`)))

(fn `F_TimerControllerToggle`
  (params (TimerForward :type Boolean))
  (bind _output_get (set `self.TimerForward` TimerForward))
  (if (not _output_get)
    (`self.F_UpdateBackwardTime`))
  (if (`KismetSystemLibrary.K2_IsValidTimerHandle` (`self.Timer Controller`))
    (`KismetSystemLibrary.K2_UnPauseTimerHandle` (`self.Timer Controller`))
    (else
      (bind _returnvalue (`KismetSystemLibrary.K2_SetTimerDelegate` (`|CreateDelegate` :!event `F_UpdateTimers`) 1.0 true))
      (set `self.Timer Controller` _returnvalue))))

(fn `F_TimerCountCalculcation`
  (if (== (`self.Sec`) 0)
    (if (== (`self.Min`) 0)
      (if (== (`self.Hour`) 0)
        (`KismetSystemLibrary.K2_ClearAndInvalidateTimerHandle` (`self.Timer Controller`))
        (else
          (set `self.Hour` (- (`self.Hour`) 1))
          (set `self.Min` 59)
          (`self.ED_Timer` (struct) :!label _label)))
      (else
        (set `self.Min` (- (`self.Min`) 1))
        (set `self.Sec` 59)
        (goto _label)))
    (else
      (set `self.Sec` (- (`self.Sec`) 1))
      (goto _label))))

(fn `F_TimerPauseController`
  (params (Toggle :type Boolean))
  (bind _timer_controller (`self.Timer Controller`))
  (if (`KismetSystemLibrary.K2_IsValidTimerHandle` (`self.Timer Controller`))
    (if Toggle
      (`KismetSystemLibrary.K2_PauseTimerHandle` _timer_controller)
      (else
        (`KismetSystemLibrary.K2_UnPauseTimerHandle` _timer_controller)))))

(fn `F_TimerReset `
  (set `self.TC_Counter` (struct))
  (`KismetSystemLibrary.K2_ClearAndInvalidateTimerHandle` (`self.Timer Controller`)))

(fn `F_UpdateBackwardTime`
  (set `self.Sec` (`self.Backward_Sec`))
  (set `self.Min` (`self.Backward_Min`))
  (set `self.Hour` (`self.Backward_Hours`)))

(fn `F_UpdateTimers`
  (if (`self.TimerForward`)
    (`self.F_ForwardTimerCalculcation`)
    (else
      (`self.F_TimerCountCalculcation`))))