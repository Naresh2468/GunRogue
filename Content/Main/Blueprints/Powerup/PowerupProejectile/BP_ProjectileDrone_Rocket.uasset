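; Rocket projectile, apparently fired by a powerup drone, that deals area damage on impact.
; When its mesh hits something, a sphere overlap trace of one object type runs at its location, ignoring the player character and drawing debug shapes.
; Each hit actor receives a damage message crediting the player as causer.
; The rocket destroys itself only if the trace finds something.
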(event `self.SM_Mesh.OnComponentHit`
  (params (HitComponent :type "PrimitiveComponent Object Reference") (OtherActor :type "Actor Object Reference") (OtherComp :type "PrimitiveComponent Object Reference") (NormalImpulse :type "Vector Structure") (Hit :type "HitResult Structure (by ref)"))
  (bind _returnvalue (`self.K2_GetActorLocation`))
  (bind (_outhits _returnvalue_2) (`KismetSystemLibrary.SphereTraceMultiForObjects` _returnvalue _returnvalue 800.0 (`|MakeArray` "ObjectTypeQuery10" :!type "EObjectTypeQuery Enum") false (`|MakeArray` (`GameplayStatics.GetPlayerCharacter` 0) :!type "Actor Object Reference") "ForDuration" true (struct :`R` 0.783026 :`G` 0.021221 :`B` 1.0 :`A` 1.0)))
  (if _returnvalue_2
    (for _array_element _outhits
      (message `/Game/Main/Blueprints/Data/Interfaces/Gameplay/HealthDamage/BPI_Damageable.F_TakeDamage` (`.HitActor` (`GameplayStatics.BreakHitResult` _array_element)) (make `/Game/Main/Blueprints/Data/Struct/Character/Damage/S_DamageInfo` 200.0 "NewEnumerator3") (`GameplayStatics.GetPlayerCharacter` 0) _array_element))
    (`self.K2_DestroyActor`)))

(fn `UserConstructionScript`
  (`parent.UserConstructionScript`))