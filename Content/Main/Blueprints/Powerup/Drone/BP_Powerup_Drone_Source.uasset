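; BP_Powerup_Drone_Source is a drone powerup Blueprint that relays rail attack triggers to the actor held in its child actor component.
; On BeginPlay it runs parent logic, then creates a looping PowerUpTimer and immediately pauses it.
; DroneAttackRail sends the IEPowerupAttackMessage to the CAHolder01 child actor, leaving the attack behavior to that actor.
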(event `self.ReceiveBeginPlay`
  (`parent.ReceiveBeginPlay`)
  (bind _returnvalue (`KismetSystemLibrary.K2_SetTimerDelegate` (`|CreateDelegate` :!event `DroneAttackRail`) 2.5 true))
  (bind _output_get (set `self.PowerUpTimer` _returnvalue))
  (`KismetSystemLibrary.K2_PauseTimerHandle` _output_get))

(event `DroneAttackRail`
  (message `/Game/Main/Blueprints/Data/Interfaces/Powerup/BPI_Powerup.IE_PowerupAttack` (`ChildActorComponent.ChildActor` (`self.CA_Holder_01`))))

(fn `UserConstructionScript`
  (`parent.UserConstructionScript`))