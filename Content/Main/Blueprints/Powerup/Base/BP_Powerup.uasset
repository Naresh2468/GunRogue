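; BP_Powerup is a base Blueprint for powerups, holding each one's info, name, default level and cooldown.
; On BeginPlay it loads that data from a data table row.
; The upgrade interface event raises the level by one, clamped to the max via a macro, prints it, then calls UpgradeElements.
; UpgradeElements and the toggle event are empty hooks, and an interface function returns the powerup info.
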(event `self.ReceiveBeginPlay`
  (bind (_dt_powerupdata_datatable _dt_powerupdata_rowname) (break `DataTableRowHandle` (`self.DT_PowerupData`)))
  (bind _returnvalue (`|GetDataTableRow` _dt_powerupdata_datatable _dt_powerupdata_rowname)
    (:`then`
      (set `self.PowerupInfo` _returnvalue)
      (bind ((`Name_2_70437F2A426B7F474748C78DB30C7229` _name) (`Level_5_59ED490440CE89CCE4EAAB89075862CE` _level) (`isUpgradeable_36_7125D42B4966B74AB87953BE3A633D2D` _isupgradeable) (`PowerupStats_20_5FCDDB9A4C04806F6233AEA6D156C381` _powerupstats)) (break `/Game/Main/Blueprints/Data/Struct/Powerup/BaseInfo/S_Powerup` _returnvalue))
      (set `self.PowerupName` _name)
      (set `self.DefaultPowerupLevel` _level)
      (set `self.DefaultCooldown` (`.Cooldown_15_8AF78C724F1DC7530965658590FB7CC1` (break `/Game/Main/Blueprints/Data/Struct/Powerup/BaseInfo/S_PowerpStats` _powerupstats))))))

(event `/Game/Main/Blueprints/Data/Interfaces/Powerup/BPI_Powerup.IE_UpgradePowerup`
  (`self.F_SetPowerupLevel`)
  (`self.UpgradeElements`))

(event `UpgradeElements`)

(event `/Game/Main/Blueprints/Data/Interfaces/Powerup/BPI_Powerup.IE_PowerupToggle`
  (params (IsActive :type Boolean)))

(fn `F_SetPowerupLevel`
  (bind _powerupinfo (`self.PowerupInfo`))
  (bind ((`Level_5_59ED490440CE89CCE4EAAB89075862CE` _level) (`MaxLevel_16_AFB3398F41C553472B5A53A8B439CD2B` _maxlevel)) (break `/Game/Main/Blueprints/Data/Struct/Powerup/BaseInfo/S_Powerup` _powerupinfo))
  (bind _result (`self.M_ClampAddition` _level _maxlevel))
  (setmembers `/Game/Main/Blueprints/Data/Struct/Powerup/BaseInfo/S_Powerup` :`StructRef` _powerupinfo :`Level` _result)
  (`KismetSystemLibrary.PrintString` (`KismetStringLibrary.Concat_StrStr` (`KismetSystemLibrary.GetDisplayName` self) (`KismetStringLibrary.Conv_IntToString` _result))))

(fn `IF_PowerupDetails`
  (returns (Powerup :type "/Game/Main/Blueprints/Data/Struct/Powerup/BaseInfo/S_Powerup Structure"))
  (return (`self.PowerupInfo`)))

(fn `UserConstructionScript`)