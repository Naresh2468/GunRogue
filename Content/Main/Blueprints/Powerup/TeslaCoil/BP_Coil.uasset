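; Tesla coil powerup that, on each IEAttack event, fires a spark beam and damages what it hits on the player's behalf.
; A wide sphere trace down the coil's axis supplies a target point; without a hit, it randomly skips or picks a random downward direction.
; A narrower trace along that ray, ignoring the player, sets the TeslaBeam endpoint and sends damage to any BPI_Damageable actor hit.
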(event `/Game/Main/Blueprints/Data/Interfaces/Powerup/BPI_CoilAttack.IE_Attack`
  (bind _sm_coil (`self.SM_Coil`))
  (bind _teslabeam (`self.TeslaBeam`))
  (bind _returnvalue (`SceneComponent.K2_GetComponentLocation` _sm_coil))
  ; Finding the enemy under the sphere detection and for checking ray direction and Distance validation of the randomness
  (set `self.Random Direction` (`self.RandomDirection`))
  (bind (_outhit _returnvalue_2) (`KismetSystemLibrary.SphereTraceSingleForObjects` _returnvalue (+ _returnvalue (* (`SceneComponent.GetUpVector` _sm_coil) -1000.0)) 100.0 (`|MakeArray` "ObjectTypeQuery10" :!type "EObjectTypeQuery Enum")))
  (bind (_start _end _randomaction) (`self.RayDirectionAndDistance` _sm_coil (`.ImpactPoint` (`GameplayStatics.BreakHitResult` _outhit)) (not _returnvalue_2)))
  (if (not _randomaction)
    ; Tesla Coil random spark effect and damage action if the enemy is detected
    (bind _outhit_2 (`KismetSystemLibrary.SphereTraceSingleForObjects` _start _end 20.0 (`|MakeArray` "ObjectTypeQuery10" "ObjectTypeQuery1" "ObjectTypeQuery2" :!type "EObjectTypeQuery Enum") false (`|MakeArray` (`GameplayStatics.GetPlayerCharacter` 0) :!type "Actor Object Reference") "ForDuration"))
    (`NiagaraComponent.ResetSystem` _teslabeam)
    (bind (_bblockinghit _binitialoverlap _time _distance _location _impactpoint _normal _impactnormal _physmat _hitactor _hitcomponent _hitbonename _bonename _hititem _elementindex _faceindex _tracestart _traceend) (`GameplayStatics.BreakHitResult` _outhit_2))
    (`NiagaraComponent.SetVariableVec3` _teslabeam "BeamEndPoint" _traceend)
    (if (`KismetSystemLibrary.DoesImplementInterface` _hitactor "/Game/Main/Blueprints/Data/Interfaces/Gameplay/HealthDamage/BPI_Damageable.BPI_Damageable_C")
      (`NiagaraComponent.SetVariableVec3` _teslabeam "ImpactNormal" _impactpoint)
      (message `/Game/Main/Blueprints/Data/Interfaces/Gameplay/HealthDamage/BPI_Damageable.F_TakeDamage` _hitactor (make `/Game/Main/Blueprints/Data/Struct/Character/Damage/S_DamageInfo` 50.0 "NewEnumerator2") (`GameplayStatics.GetPlayerCharacter` 0) _outhit_2))))

(fn `UserConstructionScript`)