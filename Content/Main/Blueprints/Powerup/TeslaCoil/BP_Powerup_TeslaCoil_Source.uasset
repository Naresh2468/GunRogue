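; Tesla Coil powerup core that attaches to the player's Powerup socket and drives two rotating child-actor rings.
; Collision overlaps track living BPI_Damageable actors, unpausing a looping attack timer on detection and pausing it when the list empties.
; Attack checks tell the rings to fire if a live target exists, with a sphere trace as fallback detection when none is found.
; Toggle and elemental upgrade events are forwarded to the rings.
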(event `self.ReceiveBeginPlay`
  ; TeslaCoil Core setup
  (`parent.ReceiveBeginPlay`)
  (`self.F_CoilCollection`)
  (bind _returnvalue (`KismetSystemLibrary.K2_SetTimerDelegate` (`|CreateDelegate` :!event `TeslaCoilAttack`) 2.0 true))
  (set `self.PowerUpTimer` _returnvalue))

(event `/Game/Main/Blueprints/Data/Interfaces/Powerup/BPI_Powerup.IE_PowerupToggle`
  (params (IsActive :type Boolean))
  ; TeslaCoil Core setup
  ;; Startup Activate
  (`parent.IE_PowerupToggle` IsActive)
  (`self.F_AttachPowerup`)
  (for _array_element (`self.Collection - RingTesla`)
    (`/Engine/EditorBlueprintResources/StandardMacros.IsValid` _array_element
      (:`Is Valid`
        (message `/Game/Main/Blueprints/Data/Interfaces/Powerup/BPI_Powerup.IE_PowerupToggle` _array_element IsActive)))))

(event `TeslaCoilAttack`
  ; TeslaCoil Core setup
  (bind _enemyalive (`self.F_ShouldAttack`))
  (if _enemyalive
    (`self.F_Attack`)))

(event `/Game/Main/Blueprints/Data/Interfaces/Powerup/BPI_Powerup.IE_UpgradeElements`
  (params (UpgradeType :type Name))
  ; TeslaCoil Core setup
  (`parent.IE_UpgradeElements` UpgradeType)
  (`self.F_UpgradeElementsRings` UpgradeType))

(event `self.Collision - Detection.OnComponentBeginOverlap`
  (params (OverlappedComponent :type "PrimitiveComponent Object Reference") (OtherActor :type "Actor Object Reference") (OtherComp :type "PrimitiveComponent Object Reference") (OtherBodyIndex :type Integer) (bFromSweep :type Boolean) (SweepResult :type "HitResult Structure (by ref)"))
  ; TeslaCoil Core setup
  (`self.F_AttackActionControl` OtherActor true))

(event `self.Collision - Detection.OnComponentEndOverlap`
  (params (OverlappedComponent :type "PrimitiveComponent Object Reference") (OtherActor :type "Actor Object Reference") (OtherComp :type "PrimitiveComponent Object Reference") (OtherBodyIndex :type Integer))
  ; TeslaCoil Core setup
  (`self.F_RemoveTarget` OtherActor))

(fn `F_AddTargets`
  (params (Target :type "Actor Object Reference"))
  (bind _actordetection (`self.ActorDetection`))
  (bind _enemyalive (message `/Game/Main/Blueprints/Data/Interfaces/Gameplay/HealthDamage/BPI_Damageable.F_GetIsAlive` Target))
  (if (and _enemyalive (not (`KismetArrayLibrary.Array_Contains` _actordetection Target)))
    (`KismetArrayLibrary.Array_Add` _actordetection Target)))

(fn `F_AttachPowerup`
  ; Attach To Player
  (if true
    ;; Testing
    (bind (_player _character) (message `/Game/Marketplace/ALS/Blueprints/Interfaces/BPI_Player.F_PlayerRef` (`GameplayStatics.GetPlayerCharacter` 0)))
    (`self.K2_AttachToComponent` self (`Character.Mesh` _character) "Powerup" "SnapToTarget" "KeepWorld" "KeepWorld" true)))

(fn `F_Attack`
  (for _array_element (`self.Collection - RingTesla`)
    (message `/Game/Main/Blueprints/Data/Interfaces/Powerup/BPI_Powerup.IE_PowerupAttack` _array_element)))

(fn `F_AttackActionControl`
  (params (Actor :type "Actor Object Reference") (Active :type Boolean))
  (if (`KismetSystemLibrary.DoesImplementInterface` Actor "/Game/Main/Blueprints/Data/Interfaces/Gameplay/HealthDamage/BPI_Damageable.BPI_Damageable_C")
    (`self.F_AddTargets` Actor)
    (if (`KismetArrayLibrary.Array_IsNotEmpty` (`self.ActorDetection`))
      (`self.F_AttackTimerController` (`local.Active`) (`self.PowerUpTimer`)))))

(fn `F_AttackTimerController`
  (params (Active :type Boolean) (`Current Powerup Handle` :type "TimerHandle Structure"))
  (if (and Active (`KismetSystemLibrary.K2_IsValidTimerHandle` (`local.Current Powerup Handle`)))
    (`KismetSystemLibrary.K2_UnPauseTimerHandle` (`local.Current Powerup Handle`))
    (else
      (`KismetSystemLibrary.K2_PauseTimerHandle` (`local.Current Powerup Handle`)))))

(fn `F_CoilCollection`
  (for (_array_element _array_index) (`|MakeArray` (`self.BP_Powerup_TeslaCoilRing_01`) (`self.BP_Powerup_TeslaCoilRing_02`))
    (bind _childactor (`ChildActorComponent.ChildActor` _array_element))
    (bind _returnvalue (`self.GetComponentByClass` _childactor "/Script/Engine.RotatingMovementComponent"))
    (`/Engine/EditorBlueprintResources/StandardMacros.IsValid` _returnvalue
      (:`Is Valid`
        (set `RotatingMovementComponent.RotationRate` (`|GetArrayItem` (`self.Rotation Rate`) _array_index) _returnvalue)
        (`KismetArrayLibrary.Array_Add` (`self.Collection - RingTesla`) _childactor)))))

(fn `F_RemoveTarget`
  (params (TargetActor :type "Actor Object Reference"))
  (bind _actordetection (`self.ActorDetection`))
  (bind _bp_enemybase (message `/Game/Main/Blueprints/Data/Interfaces/Character/Enemy/BPI_EnemyBase.F_GetEnemyBase` TargetActor))
  (if (and (== _bp_enemybase TargetActor) (`KismetArrayLibrary.Array_Contains` _actordetection _bp_enemybase))
    (`KismetArrayLibrary.Array_RemoveItem` _actordetection TargetActor)
    (if (`KismetArrayLibrary.Array_IsEmpty` _actordetection)
      (`self.F_AttackTimerController` false (`self.PowerUpTimer`)))))

(fn `F_ShouldAttack`
  (returns (EnemyAlive :type Boolean))
  (bind _returnvalue (`self.K2_GetActorLocation`))
  (for _array_element (`self.ActorDetection`)
    (`/Engine/EditorBlueprintResources/StandardMacros.IsValid` _array_element
      (:`Is Valid`
        (bind _enemyalive (message `/Game/Main/Blueprints/Data/Interfaces/Gameplay/HealthDamage/BPI_Damageable.F_GetIsAlive` _array_element))
        (if _enemyalive
          (return true)
          (else
            (`self.F_RemoveTarget` _array_element)
            (return false))))))
  (bind (_outhits _returnvalue_2) (`KismetSystemLibrary.SphereTraceMulti` _returnvalue _returnvalue 600.0 "TraceTypeQuery1"))
  (if _returnvalue_2
    (for _array_element_2 _outhits
      (`self.F_AttackActionControl` (`.HitActor` (`GameplayStatics.BreakHitResult` _array_element_2)) true))
    (else
      (`self.F_AttackTimerController` false)))
  (return false))

(fn `F_UpgradeElements`
  (params (Selection :type Name))
  (bind ((`Level_5_59ED490440CE89CCE4EAAB89075862CE` _level) (`MaxLevel_16_AFB3398F41C553472B5A53A8B439CD2B` _maxlevel)) (break `/Game/Main/Blueprints/Data/Struct/Powerup/BaseInfo/S_Powerup` (`self.PowerupInfo`)))
  (if (>= _level _maxlevel)
    (bind _output_get (set `self.CurrentUpgradeType` Selection))
    (switch `name` _output_get)
    (else
      (`KismetSystemLibrary.PrintString` "Upgarde to Level 5 " true true (struct :`R` 1.0 :`B` 0.111111 :`A` 1.0)))))

(fn `F_UpgradeElementsRings`
  (params (UpgradeName :type Name))
  (for _array_element (`|MakeArray` (`self.BP_Powerup_TeslaCoilRing_01`) (`self.BP_Powerup_TeslaCoilRing_02`))
    (bind _childactor (`ChildActorComponent.ChildActor` _array_element))
    (`/Engine/EditorBlueprintResources/StandardMacros.IsValid` _childactor
      (:`Is Valid`
        (message `/Game/Main/Blueprints/Data/Interfaces/Powerup/BPI_Powerup.IE_UpgradeElements` _childactor UpgradeName)))))

(fn `UserConstructionScript`
  (`parent.UserConstructionScript`))