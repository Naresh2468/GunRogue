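; Tesla coil ring powerup that carries a collection of coil child actors, with RotatingMovement and a looping timer both switched by the powerup toggle.
; Coils receive shock attack and upgrade calls through interface messages, with powerup info sent to the two source coils at BeginPlay.
; AddCoil spawns extra BP_Coil child components at offsets from existing ones using a wrapping index, triggered here only by an unwired debug event.
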(event `DebugUpgrades`
  (params (Selection :type Name))
  (bind _powerupinfo (`self.PowerupInfo`))
  ; Debug
  (setmembers `/Game/Main/Blueprints/Data/Struct/Powerup/BaseInfo/S_Powerup` :`StructRef` _powerupinfo :`Level` (`.MaxLevel_16_AFB3398F41C553472B5A53A8B439CD2B` (break `/Game/Main/Blueprints/Data/Struct/Powerup/BaseInfo/S_Powerup` _powerupinfo)))
  (`self.AddCoil`))

(event `self.ReceiveBeginPlay`
  (`parent.ReceiveBeginPlay`)
  (bind _returnvalue (`KismetSystemLibrary.K2_SetTimerDelegate` (`|CreateDelegate` :!event `CoilsShockAttack`) 2.5 true))
  (bind _output_get (set `self.TeslaCoilPowerUpTimer` _returnvalue))
  (`KismetSystemLibrary.K2_PauseTimerHandle` _output_get)
  (bind _output_get_2 (set `self.CoilCollection` (`|MakeArray` (`self.CA-CoilCenterSource_01`) (`self.CA-CoilCenterSource_02`))))
  (for _array_element _output_get_2
    (message `/Game/Main/Blueprints/Data/Interfaces/Powerup/BPI_CoilAttack.IE_PowerupInfo` (`ChildActorComponent.ChildActor` _array_element) (`self.PowerupInfo`))))

(event `AddCoil`
  (for _index (range (+ (`self.NumberOfCoil`) 1))
    (bind _output (`|GetArrayItem` (`self.CoilCollection`) _index))
    (bind _returnvalue (`AddComponent|NODE_AddChildActorComponent-0` :`self` self :`RelativeTransform` (`KismetMathLibrary.MakeTransform` (+ (`SceneComponent.RelativeLocation` _output) (`|GetArrayItem` (`self.OffsetCollection`) (`self.F_CurrentCoilIndex` (`|MakeArray` (`self.CA-CoilCenterSource_01`) (`self.CA-CoilCenterSource_02`))))) (`SceneComponent.RelativeRotation` _output))))
    (`ChildActorComponent.SetChildActorClass` _returnvalue "/Game/Main/Blueprints/Powerup/TeslaCoil/BP_Coil.BP_Coil_C")
    (`KismetArrayLibrary.Array_Add` (`self.CoilCollection`) _returnvalue)))

(event `CoilsShockAttack`
  (for _array_element (`self.CoilCollection`)
    (bind _childactor (`ChildActorComponent.ChildActor` _array_element))
    (`/Engine/EditorBlueprintResources/StandardMacros.IsValid` _childactor
      (:`Is Valid`
        (message `/Game/Main/Blueprints/Data/Interfaces/Powerup/BPI_CoilAttack.IE_Attack` _childactor)))))

(event `self.UpgradeElements`
  (`parent.UpgradeElements`))

(event `/Game/Main/Blueprints/Data/Interfaces/Powerup/BPI_Powerup.IE_PowerupToggle`
  (params (IsActive :type Boolean))
  (bind _teslacoilpoweruptimer (`self.TeslaCoilPowerUpTimer`))
  (bind _rotatingmovement (`self.RotatingMovement`))
  (if IsActive
    (`KismetSystemLibrary.K2_UnPauseTimerHandle` _teslacoilpoweruptimer)
    (`ActorComponent.SetComponentTickEnabled` _rotatingmovement true)
    (else
      (`KismetSystemLibrary.K2_PauseTimerHandle` _teslacoilpoweruptimer)
      (`ActorComponent.SetComponentTickEnabled` _rotatingmovement false))))

(event `/Game/Main/Blueprints/Data/Interfaces/Powerup/BPI_Powerup.IE_UpgradeElements`
  (params (UpgradeType :type Name))
  (`self.F_CoilUpgrade` UpgradeType))

(fn `F_CoilUpgrade`
  (params (Upgrade :type Name))
  (for _array_element (`self.CoilCollection`)
    (bind _childactor (`ChildActorComponent.ChildActor` _array_element))
    (`/Engine/EditorBlueprintResources/StandardMacros.IsValid` _childactor
      (:`Is Valid`
        (message `/Game/Main/Blueprints/Data/Interfaces/Powerup/BPI_CoilAttack.IE_PowerupUpgradeElementsCoils` _childactor Upgrade)))))

(fn `F_CurrentCoilIndex`
  (params (TargetArray :type "Array of ChildActorComponent Object Reference (by ref)"))
  (returns (Count :type Integer))
  (bind _currentcoilringcount (`self.CurrentCoilRingCount`))
  (bind _output_get (set `self.CurrentCoilRingCount` (`KismetMathLibrary.SelectInt` 0 (+ _currentcoilringcount 1) (>= _currentcoilringcount (`KismetArrayLibrary.Array_LastIndex` TargetArray)))))
  (return _output_get))

(fn `F_Location`
  (params (Index :type Integer) (Total :type Integer))
  (returns (Output_Get :type "Vector Structure"))
  (bind _output_get (set `self.Radian` (`KismetMathLibrary.DegreesToRadians` (`KismetMathLibrary.Conv_IntToDouble` (* Index (/ 360 Total))))))
  (bind _output_get_2 (set `self.Location` (`KismetMathLibrary.MakeVector` (* (`KismetMathLibrary.Cos` _output_get) 30.0) (* (`KismetMathLibrary.Sin` _output_get) 30.0))))
  (return _output_get_2))

(fn `UserConstructionScript`
  (`parent.UserConstructionScript`))