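; Spectator pawn for the VR player, providing free-flight movement until spectating is toggled off.
; SetupSpectator stores the VR pawn, adds the spectator Enhanced Input mapping context and resets HMD orientation and position.
; Move input strafes horizontally and flies along the full camera forward vector, while turn input adds controller yaw, both scaled by Pace.
; The toggle action removes the mapping, repossesses the VR player, restores its controls and destroys this pawn.
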(event `SetupSpectator`
  (params (BP_VRPlayer :type "/Game/Main/Blueprints/Character/Player/BP_VRCharacter Object Reference"))
  (set `self.BP_VRPlayer` BP_VRPlayer)
  (`self.F_Input` true)
  (`HeadMountedDisplayFunctionLibrary.ResetOrientationAndPosition` 0.0))

(event `EnhancedInput|/Game/Main/Blueprints/Data/Input/Actions/Spectator/IA_SpectatorToggle`
  (params (ActionValue :type Boolean) (ElapsedSeconds :type "Float (double-precision)") (TriggeredSeconds :type "Float (double-precision)") (InputAction :type "InputAction Object Reference" :default "/Game/Main/Blueprints/Data/Input/Actions/Spectator/IA_SpectatorToggle.IA_SpectatorToggle"))
  (bind _bp_vrplayer (`self.BP_VRPlayer`))
  (:`Started`
    (`self.F_Input` false)
    (`Controller.Possess` (`GameplayStatics.GetPlayerController` 0) _bp_vrplayer)
    (`/Game/Main/Blueprints/Character/Player/BP_VRCharacter.F_PlayerInputControlling` _bp_vrplayer)
    (`self.K2_DestroyActor`)))

(event `EnhancedInput|/Game/Main/Blueprints/Data/Input/Actions/Spectator/IA_SpectatorTurn`
  (params (ActionValue :type "Vector2D Structure") (ElapsedSeconds :type "Float (double-precision)") (TriggeredSeconds :type "Float (double-precision)") (InputAction :type "InputAction Object Reference" :default "/Game/Main/Blueprints/Data/Input/Actions/Spectator/IA_SpectatorTurn.IA_SpectatorTurn"))
  (:`Triggered`
    (`self.AddControllerYawInput` (* ActionValue_X (`self.Pace`)))))

(event `EnhancedInput|/Game/Main/Blueprints/Data/Input/Actions/Spectator/IA_SpectatorMove`
  (params (ActionValue :type "Vector2D Structure") (ElapsedSeconds :type "Float (double-precision)") (TriggeredSeconds :type "Float (double-precision)") (InputAction :type "InputAction Object Reference" :default "/Game/Main/Blueprints/Data/Input/Actions/Spectator/IA_SpectatorMove.IA_SpectatorMove"))
  (bind (_returnvalue_x _returnvalue_y) (`KismetMathLibrary.BreakVector` (`self.GetActorRightVector` (`GameplayStatics.GetPlayerCameraManager` 0))))
  (bind (_returnvalue_x_2 _returnvalue_y_2 _returnvalue_z) (`KismetMathLibrary.BreakVector` (`self.GetActorForwardVector` (`GameplayStatics.GetPlayerCameraManager` 0))))
  (:`Triggered`
    (`self.AddMovementInput` (`KismetMathLibrary.MakeVector` _returnvalue_x _returnvalue_y) (* ActionValue_X (`self.Pace`)))
    (`self.AddMovementInput` (`KismetMathLibrary.MakeVector` _returnvalue_x_2 _returnvalue_y_2 _returnvalue_z) (* ActionValue_Y (`self.Pace`)))))

(fn `F_Input`
  (params (Input :type Boolean))
  (bind _returnvalue (`GameplayStatics.GetPlayerController` 0))
  (if Input
    (bind _asbp_game_controller (cast `/Game/Main/Blueprints/Data/Controller/BP_GameController` _returnvalue))
    (set `self.As BP Game Controller` _asbp_game_controller)
    (`EnhancedInputSubsystemInterface.AddMappingContext` (pcsubsystem `EnhancedInputLocalPlayerSubsystem` _asbp_game_controller) "/Game/Main/Blueprints/Data/Input/Mapping/IMC_VRPlayerSpectator.IMC_VRPlayerSpectator" 0 (struct))
    (`self.EnableInput` _returnvalue)
    (else
      (`EnhancedInputSubsystemInterface.RemoveMappingContext` (pcsubsystem `EnhancedInputLocalPlayerSubsystem` (`self.As BP Game Controller`)) "/Game/Main/Blueprints/Data/Input/Mapping/IMC_VRPlayerSpectator.IMC_VRPlayerSpectator" (struct))
      (`self.DisableInput` (`GameplayStatics.GetPlayerController` 0)))))

(fn `UserConstructionScript`)