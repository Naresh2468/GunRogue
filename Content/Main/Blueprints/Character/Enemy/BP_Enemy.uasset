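; BP_Enemy is an enemy character that routes damage, healing and health queries to its BP_HealthComponent.
; Getters expose attack/defend ranges, and movement type sets walk speed.
; Damage spawns an impact effect; death stops AI logic, ragdolls the mesh with a backward impulse, then destroys the actor after a delay.
; Attack only prints and token reservation always fails; separate helpers tune projectile homing by target distance.
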(event `self.ReceiveBeginPlay`)

(event `/Game/Main/Blueprints/Data/Interfaces/Character/Enemy/BPI_EnemyBase.IE_Attack`
  (params (AttackTarget :type "Actor Object Reference"))
  (`KismetSystemLibrary.PrintString` "Attacking"))

(event `self.BP_HealthComponent.OnDeath`
  (bind _mesh (`self.Mesh`))
  (`BrainComponent.StopLogic` (`AIController.BrainComponent` (`self.AIC_EnemyBase`)) "Death")
  (`PrimitiveComponent.SetCollisionEnabled` (`self.CapsuleComponent`) "NoCollision")
  (`PrimitiveComponent.SetCollisionEnabled` _mesh "QueryAndPhysics")
  (`PrimitiveComponent.SetSimulatePhysics` _mesh true)
  (`PrimitiveComponent.AddImpulse` _mesh (* (`self.GetActorForwardVector`) -200.0) "None" true)
  (`KismetSystemLibrary.Delay` 5.0)
  (`self.K2_DestroyActor`))

(event `self.BP_HealthComponent.OnTakeDamage`
  (`GameplayStatics.SpawnEmitterAtLocation` "/Game/Marketplace/Weapon/MilitaryWeapDark/FX/P_Impact_Metal_Medium_01.P_Impact_Metal_Medium_01" (`self.K2_GetActorLocation`) (struct) (4.0 4.0 4.0)))

(fn `F_GetCurrentHealth`
  (returns (Value :type "Float (double-precision)"))
  (return (`/Game/Marketplace/ALS/Blueprints/Components/BP_HealthComponent.CurrentHealth` (`self.BP_HealthComponent`))))

(fn `F_GetEnemyBase`
  (returns (BP_EnemyBase :type "/Game/Main/Blueprints/Character/Enemy/BP_Enemy Object Reference"))
  (return self))

(fn `F_GetIdealRange`
  (returns (AttackRadius :type "Float (double-precision)") (DefendRadius :type "Float (double-precision)"))
  (return (`self.Attack Radius`) (`self.Defend Radius`)))

(fn `F_GetMaxHealth`
  (returns (Value :type "Float (double-precision)"))
  (return (`/Game/Marketplace/ALS/Blueprints/Components/BP_HealthComponent.MaxHealth` (`self.BP_HealthComponent`))))

(fn `F_HealProcess`
  (params (Amount :type "Float (double-precision)"))
  (returns (Value :type "Float (double-precision)"))
  (bind _healthvalue (`/Game/Marketplace/ALS/Blueprints/Components/BP_HealthComponent.F_Heal` (`self.BP_HealthComponent`) Amount))
  (return _healthvalue))

(fn `F_HomingMotion`
  (bind _projectilemovement (`self.ProjectileMovement`))
  (bind _returnvalue (< (`KismetMathLibrary.Vector_Distance` (`SceneComponent.K2_GetComponentLocation` (`self.TargetComponent`)) (`self.K2_GetActorLocation`)) 500.0))
  (`self.TargetComponent`
    (:`then`
      (set `ProjectileMovementComponent.HomingAccelerationMagnitude` (select `bool` _returnvalue :`false` (`self.Homing Acceleration Magnitude`) :`true` (* (`self.Homing Acceleration Magnitude`) 2.5) :!type "Float (single-precision)") _projectilemovement)
      (set `ProjectileMovementComponent.bIsHomingProjectile` (not _returnvalue) _projectilemovement)
      (set `ProjectileMovementComponent.ProjectileGravityScale` (select `bool` _returnvalue :`false` 0.8 :`true` -0.2 :!type "Float (single-precision)") _projectilemovement))
    (:`else`)))

(fn `F_IsDeath`
  (returns (isDeath :type Boolean))
  (return (`/Game/Marketplace/ALS/Blueprints/Components/BP_HealthComponent.IsDead?` (`self.BP_HealthComponent`))))

(fn `F_ReserveAttackToken`
  (params (Amount :type Integer))
  (returns (Sucess :type Boolean))
  (return false))

(fn `F_Set_MovementSpeed`
  (params (MovmentType :type "/Game/Main/Blueprints/Data/Enum/Character/Movement/E_Movement Enum" :default "NewEnumerator0"))
  (returns (SpeedValue :type "Float (double-precision)"))
  (bind _output_get (set `CharacterMovementComponent.MaxWalkSpeed` (select `/Game/Main/Blueprints/Data/Enum/Character/Movement/E_Movement` MovmentType :`NewEnumerator1` 100.0 :`NewEnumerator2` 250.0 :`NewEnumerator4` 300.0) (`self.CharacterMovement`)))
  (return _output_get))

(fn `F_SetHoming`
  (params (Actor :type "Actor Object Reference"))
  (bind _returnvalue (select `bool` (`KismetSystemLibrary.IsValid` Actor) :`false` (`self.Direction`) :`true` (`self.GetComponentByClass` Actor "/Script/Engine.ArrowComponent")))
  (`/Engine/EditorBlueprintResources/StandardMacros.IsValid` Actor
    (:`Is Valid`
      (set `self.TargetComponent` _returnvalue)
      (set `ProjectileMovementComponent.HomingTargetComponent` _returnvalue (`self.ProjectileMovement`)))))

(fn `F_TakeDamage`
  (params (DamageInfo :type "/Game/Main/Blueprints/Data/Struct/Character/Damage/S_DamageInfo Structure") (DamageCausor :type "Actor Object Reference") (Hit :type "HitResult Structure"))
  (returns (IsDamaged :type Boolean))
  (bind (_dead_ _damage) (`/Game/Marketplace/ALS/Blueprints/Components/BP_HealthComponent.TakeDamage` (`self.BP_HealthComponent`) (`.Amount_8_69D2C9B245A38DBF14ADBB9A6894520C` (break `/Game/Main/Blueprints/Data/Struct/Character/Damage/S_DamageInfo` DamageInfo)) (0.0 0.0 0.0) (`.HitBoneName` (`GameplayStatics.BreakHitResult` Hit)) DamageCausor))
  (return _damage))

(fn `UserConstructionScript`)